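; BP_FlappyCamera is a side-following camera actor that also spawns the Flappy player at its own transform.
; On BeginPlay it records the spawn location, possesses the spawned actor with player controller 0 and activates its Camera, printing a debug string if the Pawn cast fails.
; Each Tick it copies only the player's Y position, keeping X and Z locked to the spawn point.
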(event `self.ReceiveBeginPlay`
  (bind _returnvalue (`|SpawnActorFromClass` (`self.FlappyActor`) (`self.GetTransform`) "Undefined" "OverrideRootScale" null null))
  (bind _output_get (set `self.FlappyActorInstance` _returnvalue))
  (bind _returnvalue_location (`KismetMathLibrary.BreakTransform` (`self.GetTransform` _output_get)))
  (bind _output_get_2 (set `self.SpawnPosition` _returnvalue_location))
  (`self.K2_SetActorTransform` (`KismetMathLibrary.MakeTransform` _output_get_2))
  (bind _aspawn (cast `Pawn` (`self.FlappyActorInstance`))
    (:`then`
      (`Controller.Possess` (`GameplayStatics.GetPlayerController` 0) _aspawn)
      (`ActorComponent.Activate` (`self.Camera`) false))
    (:`CastFailed`
      (`KismetSystemLibrary.PrintString` "Hello"))))

(event `self.ReceiveActorBeginOverlap`
  (params (OtherActor :type "Actor Object Reference")))

(event `self.ReceiveTick`
  (params (DeltaSeconds :type "Float (single-precision)"))
  (bind _spawnposition_x (`KismetMathLibrary.BreakVector` (`self.SpawnPosition`)))
  (bind (_spawnposition_x_2 _spawnposition_y _spawnposition_z) (`KismetMathLibrary.BreakVector` (`self.SpawnPosition`)))
  (`self.K2_SetActorTransform` (`KismetMathLibrary.MakeTransform` (`KismetMathLibrary.MakeVector` _spawnposition_x (.y (.location (`self.GetTransform` (`self.FlappyActorInstance`)))) _spawnposition_z))))

(fn `UserConstructionScript`)