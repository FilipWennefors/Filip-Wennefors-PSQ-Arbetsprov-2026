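; Player-controlled Flappy Bird-style actor that moves forward along Y, falls under custom gravity and flaps upward on Enhanced Input jump.
; BeginPlay adds the input mapping and spawns an independent camera that Tick moves along Y only.
; Game mode start, death and respawn events set a state enum that gates movement.
; Tick applies vertical velocity per frame without delta-time scaling, while forward speed and gravity are scaled.
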(event `self.ReceiveBeginPlay`
  (bind (_returnvalue_location _returnvalue_rotation _returnvalue_scale) (`KismetMathLibrary.BreakTransform` (`self.GetTransform`)))
  (bind _returnvalue (`GameplayStatics.GetPlayerController` 0))
  ;[0 0 0] Add Inputs
  (`self.EnableInput` _returnvalue)
  (`EnhancedInputSubsystemInterface.AddMappingContext` (pcsubsystem `EnhancedInputLocalPlayerSubsystem` _returnvalue) "/Game/FlappyMappingContext.FlappyMappingContext" 0 (struct))
  ;[0 0 0] Makes Independent Camera
  (bind _returnvalue_2 (`|SpawnActorFromClass` "/Script/Engine.CameraActor" (`KismetMathLibrary.MakeTransform` (+ (`self.CamPosOffset`) _returnvalue_location) _returnvalue_rotation _returnvalue_scale) "AlwaysSpawn" "OverrideRootScale" null null))
  (bind _output_get (set `self.Flappy Camera` _returnvalue_2))
  (`PlayerController.SetViewTargetWithBlend` (`GameplayStatics.GetPlayerController` 0) _output_get 0.0 "VTBlend_Linear" 0.0 false)
  (bind _asbp_flappy_game_mode (cast `/Game/BP_FlappyGameMode` (`GameplayStatics.GetGameMode`)))
  (add `/Game/BP_FlappyGameMode.OnFlappyStartGame` _asbp_flappy_game_mode (delegate `OnFlappyStartGame`))
  (add `/Game/BP_FlappyGameMode.OnFlappyDeath` _asbp_flappy_game_mode (delegate `OnFlappyDeceased`))
  (add `/Game/BP_FlappyGameMode.OnFlappyRespawn` _asbp_flappy_game_mode (delegate `OnFlappyRespawned`)))

(event `OnFlappyStartGame`
  (set `self.FlappyStateEnum` "NewEnumerator1"))

(event `OnFlappyDeceased`
  (set `self.FlappyStateEnum` "NewEnumerator2"))

(event `OnFlappyRespawned`
  (set `self.FlappyStateEnum` "NewEnumerator1")
  (set `self.FlappyVerticalVelocity` 0.0))

(event `self.ReceiveTick`
  (params (DeltaSeconds :type "Float (single-precision)"))
  (bind (_camposoffset_x _camposoffset_y) (`KismetMathLibrary.BreakVector` (`self.CamPosOffset`)))
  (bind _returnvalue (`self.GetTransform` (`self.Flappy Camera`)))
  ;[0 0 0] Move Flappy
  (set `self.Delta Seconds` DeltaSeconds)
  (switch `/Game/E_FlappyState` (`self.FlappyStateEnum`)
    (:`NewEnumerator1`
      (`self.K2_AddActorWorldTransform` (`KismetMathLibrary.MakeTransform` (`KismetMathLibrary.MakeVector` 0.0 (* (`self.MoveSpeed`) (`self.Delta Seconds`)) (`self.FlappyVerticalVelocity`))) true)
      (set `self.FlappyVerticalVelocity` (- (`self.FlappyVerticalVelocity`) (* (`self.FlappyFallStrength`) (`self.Delta Seconds`))))
      ;[0 0 0] Move Camera
      (`self.K2_SetActorTransform` (`self.Flappy Camera`) (`KismetMathLibrary.MakeTransform` (`KismetMathLibrary.MakeVector` (.x (.location _returnvalue)) (+ (.y (.location (`self.GetTransform`))) _camposoffset_y) (.z (.location _returnvalue))) (.rotation _returnvalue) (.scale _returnvalue)) false false))))

(event `EnhancedInput|/Game/FlappyJump`
  (params (ActionValue :type Boolean) (ElapsedSeconds :type "Float (double-precision)") (TriggeredSeconds :type "Float (double-precision)") (InputAction :type "InputAction Object Reference" :default "/Game/FlappyJump.FlappyJump"))
  ;[0 0 0] Move Flappy
  (:`Triggered`
    (set `self.FlappyVerticalVelocity` (* (`self.Flappy Jump Strength`) 1.0))))

(event `EnhancedInput|/Game/FlappyJump`
  (params (ActionValue :type Boolean) (ElapsedSeconds :type "Float (double-precision)") (TriggeredSeconds :type "Float (double-precision)") (InputAction :type "InputAction Object Reference" :default "/Game/FlappyJump.FlappyJump"))
  ;[0.1771 0 0] Bugged Move code
)

(fn `ResetCameraPosition`
  (bind _returnvalue_location (`KismetMathLibrary.BreakTransform` (`self.GetTransform`)))
  (`self.K2_SetActorLocation` (`self.Flappy Camera`) (+ (`self.CamPosOffset`) _returnvalue_location) false false))

(fn `UserConstructionScript`)