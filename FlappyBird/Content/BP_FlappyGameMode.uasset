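; Game mode for a Flappy Bird-style game that spawns pipes, tracks score and signals start, death and respawn through event dispatchers.
; BeginPlay spawns a flagged first pipe and creates the HUD, which displays the score.
; Tick projects the last pipe to screen space, chaining randomly offset pipes as it nears view; off-screen cleanup is unwired.
; Reset clears score, returns the bird to PlayerStart and destroys all but the first pipe.
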(event `self.ReceiveBeginPlay`
  (`self.SpawnFirstPipe`)
  (bind _returnvalue (`|CreateWidget` "/Game/UI_Widgets/BP_FlappyGameHud.BP_FlappyGameHud_C"))
  (bind _output_get (set `self.FlappyUIReference` _returnvalue))
  (`UserWidget.AddToViewport` _output_get 0))

(event `self.ReceiveTick`
  (params (DeltaSeconds :type "Float (single-precision)"))
  (bind _nextpipespawnpos (`self.NextPipeSpawnPos`))
  (bind _returnvalue_location (`KismetMathLibrary.BreakTransform` (`self.GetTransform` (`self.Last Spawned Pipe`))))
  ;[0 0 0] Check if pipe is on screen
  (bind _returnvalue (`GameUserSettings.GetGameUserSettings`))
  (if (`KismetSystemLibrary.IsValid` (`self.Last Spawned Pipe`))
    (bind _returnvalue_x (break `IntPoint` (`GameUserSettings.GetScreenResolution` _returnvalue)))
    (if (<= (+ (`KismetMathLibrary.BreakVector2D` (`PlayerController.ProjectWorldLocationToScreen` (`GameplayStatics.GetPlayerController` 0) _returnvalue_location false)) 200.0) _returnvalue_x)
      ;[0 0 0] Spawn Next Pipe
      (bind _output_get (set `self.NextPipeSpawnPos` (`KismetMathLibrary.MakeTransform` (`KismetMathLibrary.MakeVector` (.x (.location _nextpipespawnpos)) (+ (.y (.location _nextpipespawnpos)) (`KismetMathLibrary.RandomFloatInRange` (`self.MinDistBetweenPipes`) (`self.MaxDistBetweenPipes`))) (`KismetMathLibrary.RandomFloatInRange` (`self.MinVerticalPos`) (`self.MaxVerticalPos`))) (.rotation _nextpipespawnpos) (.scale _nextpipespawnpos))))
      (bind _returnvalue_2 (`|SpawnActorFromClass` "/Game/BP_Pipes.BP_Pipes_C" _output_get "Undefined" "OverrideRootScale" null null))
      (bind _output_get_2 (set `self.Last Spawned Pipe` _returnvalue_2))
      (`KismetArrayLibrary.Array_Add` (`self.FlappyPipesArray`) _output_get_2))))

(fn `FlappyBirdPassedPipe`
  (bind _output_get (set `self.Score` (+ (`self.Score`) (`self.ScorePerPipePassed`))))
  (`/Game/UI_Widgets/UI_FlappyBirdScore.SetHighScoreNumber` (`/Game/UI_Widgets/BP_FlappyGameHud.FlappyBirdScore` (`self.FlappyUIReference`)) _output_get))

(fn `FlappyStartPlay`
  (`self.OnFlappyStartGame`))

(fn `KillFlappy`
  (`self.OnFlappyDeath`))

(fn `Reset Game`
  (`|ExecutionSequence`
    (:`then_0`
      (set `self.Score` 0)
      (`self.K2_SetActorTransform` (`GameplayStatics.GetPlayerPawn` 0) (`self.GetTransform` (`self.K2_FindPlayerStart` (`GameplayStatics.GetPlayerController` 0))) false true)
      (bind _asbp_v2flappy (cast `/Game/BP_V2Flappy` (`GameplayStatics.GetPlayerPawn` 0)))
      (`/Game/BP_V2Flappy.ResetCameraPosition` _asbp_v2flappy))
    (:`then_1`
      (set `self.Last Spawned Pipe` (`|GetArrayItem` (`self.FlappyPipesArray`))))
    (:`then_2`
      (bind (_arrayindex _arrayelement) (`/Engine/EditorBlueprintResources/StandardMacros.ReverseForEachLoop` (`self.FlappyPipesArray`))
        (:`LoopBody`
          (if (`/Game/BP_Pipes.IsFirstPipe` _arrayelement)
            (set `self.Last Spawned Pipe` _arrayelement)
            (set `self.NextPipeSpawnPos` (`self.FirstPipeSpawnPos`))
            (else
              (`self.K2_DestroyActor` _arrayelement)
              (`KismetArrayLibrary.Array_Remove` (`self.FlappyPipesArray`) _arrayindex))))
        (:`Completed`
          (`KismetSystemLibrary.PrintString` "Completeted for loop" true true (struct :`G` 0.66 :`B` 1.0 :`A` 1.0) 1000.0)
          (`KismetSystemLibrary.PrintString` (`KismetStringLibrary.BuildString_Name` "Last spawned pipe is named" "" (`KismetStringLibrary.Conv_StringToName` (`KismetSystemLibrary.GetDisplayName` (`self.Last Spawned Pipe`)))) true true (struct :`G` 0.66 :`B` 1.0 :`A` 1.0) 1000.0)
          (`self.OnFlappyRespawn`))))))

(fn `SpawnFirstPipe`
  (returns (`Spawned Pipe Reference` :type "/Game/BP_Pipes Object Reference"))
  (locals (NewLocalVar :type String :default "Pipe spawned is: "))
  (set `self.NextPipeSpawnPos` (`self.FirstPipeSpawnPos`))
  (`KismetSystemLibrary.PrintString` "Hello")
  (bind _returnvalue (`|SpawnActorFromClass` "/Game/BP_Pipes.BP_Pipes_C" (`self.NextPipeSpawnPos`) "Undefined" "OverrideRootScale" null null))
  (set `/Game/BP_Pipes.IsFirstPipe` true _returnvalue)
  (bind _output_get (set `self.Last Spawned Pipe` _returnvalue))
  (`KismetArrayLibrary.Array_Add` (`self.FlappyPipesArray`) _output_get)
  (return null))

(fn `UserConstructionScript`)