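; First-person movement actor that walks on the horizontal plane and looks around with the mouse through Enhanced Input.
; BeginPlay enables input for player zero and adds the FPMovement mapping context.
; Movement normalizes camera-relative input in XY, scales it by speed and Tick's cached delta time, then sets the actor transform directly.
; Mouse look accumulates unclamped pitch and yaw onto the camera alone, held at a fixed height.
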(event `self.ReceiveBeginPlay`
  (bind _returnvalue (`GameplayStatics.GetPlayerController` 0))
  ;[0 0 0] Add movement input
  (`self.EnableInput` _returnvalue)
  (`EnhancedInputSubsystemInterface.AddMappingContext` (pcsubsystem `EnhancedInputLocalPlayerSubsystem` _returnvalue) "/Game/Input/FPMovement.FPMovement" 0 (struct)))

(event `self.ReceiveActorBeginOverlap`
  (params (OtherActor :type "Actor Object Reference"))
  ;[0 0 0] Add movement input
)

(event `self.ReceiveTick`
  (params (DeltaSeconds :type "Float (single-precision)"))
  ;[0 0 0] Add movement input
  (set `self.Delta Seconds` DeltaSeconds))

(event `EnhancedInput|/Game/Input/PlayerMovement`
  (params (ActionValue :type "Vector2D Structure") (ElapsedSeconds :type "Float (double-precision)") (TriggeredSeconds :type "Float (double-precision)") (InputAction :type "InputAction Object Reference" :default "/Game/Input/PlayerMovement.PlayerMovement"))
  (bind _returnvalue_location (`KismetMathLibrary.BreakTransform` (`self.GetTransform`)))
  (bind (_returnvalue_x _returnvalue_y) (`KismetMathLibrary.BreakVector` (+ (* ActionValue_X (`SceneComponent.GetForwardVector` (`self.Camera`))) (* ActionValue_Y (`SceneComponent.GetRightVector` (`self.Camera`))))))
  (bind (_returnvalue_x_2 _returnvalue_y_2) (`KismetMathLibrary.BreakVector` (`KismetMathLibrary.Normal` (`KismetMathLibrary.MakeVector` _returnvalue_x _returnvalue_y))))
  ;[0 0 0] Player Movement
  (:`Triggered`
    (set `self.DeltaPosition` (`KismetMathLibrary.MakeVector` (* (`self.Delta Seconds`) (* _returnvalue_x_2 (`self.MoveSpeed`))) (* (`self.Delta Seconds`) (* _returnvalue_y_2 (`self.MoveSpeed`)))))
    (`self.K2_SetActorTransform` (`KismetMathLibrary.MakeTransform` (+ (`self.DeltaPosition`) _returnvalue_location)))))

(event `EnhancedInput|/Game/Input/MouseLook`
  (params (ActionValue :type "Vector2D Structure") (ElapsedSeconds :type "Float (double-precision)") (TriggeredSeconds :type "Float (double-precision)") (InputAction :type "InputAction Object Reference" :default "/Game/Input/MouseLook.MouseLook"))
  (bind (_camera_rot_vector_x _camera_rot_vector_y _camera_rot_vector_z) (`KismetMathLibrary.BreakVector` (`self.Camera Rot Vector`)))
  (bind _mousesensitivity (`self.MouseSensitivity`))
  (bind (_camera_rot_vector_x_2 _camera_rot_vector_y_2 _camera_rot_vector_z_2) (`KismetMathLibrary.BreakVector` (`self.Camera Rot Vector`)))
  ;[0 0 0] CameraMovement
  (:`Triggered`
    (set `self.Camera Rot Vector` (`KismetMathLibrary.MakeVector` 0.0 (+ _camera_rot_vector_y (* ActionValue_Y _mousesensitivity)) (+ _camera_rot_vector_z (* ActionValue_X _mousesensitivity))))
    (`SceneComponent.K2_SetRelativeTransform` (`self.Camera`) (`KismetMathLibrary.MakeTransform` (0.0 0.0 180.0) (`KismetMathLibrary.MakeRotator` _camera_rot_vector_x_2 _camera_rot_vector_y_2 _camera_rot_vector_z_2)) false false)))

(fn `UserConstructionScript`)