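; Pipe-pair obstacle for a Flappy Bird-style game that randomizes its gap by setting the upper pipe's relative height on BeginPlay.
; Overlaps on the score hitbox, except by its own pipes, report a pass to BP_FlappyGameMode, while player hits on either pipe call KillFlappy there.
; Off-screen deletion, respawn cleanup and hitbox-visualizer fitting via the two helper functions exist only as disconnected logic that never runs.
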(event `self.ReceiveBeginPlay`
  (bind _returnvalue (`SceneComponent.GetRelativeTransform` (`self.Upper Pipe`)))
  ;[0 0 0] Set Upper Pipe position
  (`SceneComponent.K2_SetRelativeTransform` (`self.Upper Pipe`) (`KismetMathLibrary.MakeTransform` (`KismetMathLibrary.MakeVector` (.x (.location _returnvalue)) (.y (.location _returnvalue)) (`KismetMathLibrary.RandomFloatInRange` (`self.MinDistBetweenPipes`) (`self.MaxDistBetweenPipes`))) (.rotation _returnvalue) (.scale _returnvalue)) false false))

(event `OnFlappyRespawn`)

(event `self.ReceiveTick`
  (params (DeltaSeconds :type "Float (single-precision)"))
  ;[0 0 0] Delete if out of bounds
)

(event `self.Give Score Hitbox.OnComponentBeginOverlap`
  (params (OverlappedComponent :type "PrimitiveComponent Object Reference") (OtherActor :type "Actor Object Reference") (OtherComp :type "PrimitiveComponent Object Reference") (OtherBodyIndex :type Integer) (bFromSweep :type Boolean) (SweepResult :type "HitResult Structure (by ref)"))
  ;[0 0 0] Add Score When Passing Pipe
  (if (!= OtherComp (`self.Upper Pipe`))
    (if (!= OtherComp (`self.Lower Pipe`))
      (bind _asbp_flappy_game_mode (cast `/Game/BP_FlappyGameMode` (`GameplayStatics.GetGameMode`)))
      (`/Game/BP_FlappyGameMode.FlappyBirdPassedPipe` _asbp_flappy_game_mode))))

(event `self.Lower Pipe.OnComponentHit`
  (params (HitComponent :type "PrimitiveComponent Object Reference") (OtherActor :type "Actor Object Reference") (OtherComp :type "PrimitiveComponent Object Reference") (NormalImpulse :type "Vector Structure") (Hit :type "HitResult Structure (by ref)"))
  ;[0 0 0] Kill Flappy if collision
  (if (== OtherActor (`GameplayStatics.GetPlayerPawn` 0))
    (bind _asbp_flappy_game_mode (cast `/Game/BP_FlappyGameMode` (`GameplayStatics.GetGameMode`) :!label _label))
    (`/Game/BP_FlappyGameMode.KillFlappy` _asbp_flappy_game_mode)))

(event `self.Upper Pipe.OnComponentHit`
  (params (HitComponent :type "PrimitiveComponent Object Reference") (OtherActor :type "Actor Object Reference") (OtherComp :type "PrimitiveComponent Object Reference") (NormalImpulse :type "Vector Structure") (Hit :type "HitResult Structure (by ref)"))
  ;[0 0 0] Kill Flappy if collision
  (if (== OtherActor (`GameplayStatics.GetPlayerPawn` 0))
    (goto _label)))

(fn `CalcHitboxScaleToUnitFactor`
  (returns (ScaleToUnitFactor :type "Float (double-precision)"))
  (bind (_min _max) (`StaticMeshComponent.GetLocalBounds` (`self.Hitbox visualizer`)))
  (return (/ (.z (.scale (`SceneComponent.K2_GetComponentToWorld` (`self.Hitbox visualizer`)))) (+ (`KismetMathLibrary.Abs` (.z _min)) (`KismetMathLibrary.Abs` (.z _max))))))

(fn `MoveHitboxBetweenPipes`
  (bind _returnvalue (`SceneComponent.K2_GetComponentToWorld` (`self.Lower Pipe`)))
  ;[0 0 0] Move Hitbox to middle between pipes
  (set `self.Upper pipe location` (.z (.location (`SceneComponent.K2_GetComponentToWorld` (`self.Upper Pipe`)))))
  (set `self.Lower Pipe Location` (.z (.location (`SceneComponent.K2_GetComponentToWorld` (`self.Lower Pipe`)))))
  (set `self.DistBetweenPipes` (- (`self.Upper pipe location`) (`self.Lower Pipe Location`)))
  (`SceneComponent.K2_SetWorldTransform` (`self.Hitbox visualizer`) (`KismetMathLibrary.MakeTransform` (`KismetMathLibrary.MakeVector` (.x (.location _returnvalue)) (.y (.location _returnvalue)) (+ (/ (`self.DistBetweenPipes`) 2.0) (`self.Lower Pipe Location`))) (.rotation _returnvalue) (.scale _returnvalue)) false false))

(fn `UserConstructionScript`)