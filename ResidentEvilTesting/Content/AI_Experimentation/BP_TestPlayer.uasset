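; BP_TestPlayer is an AI experimentation player that makes noise events at positions aimed with the mouse.
; BeginPlay adds the player controls input mapping context and shows the cursor.
; FireWeapon runs a debug-drawn visibility trace from the controlled pawn's location toward a far point along the deprojected cursor ray.
; The hit location receives a ranged ReportNoiseEvent, instigated by the player, and an explosion sound.
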(event `self.ReceiveBeginPlay`
  (bind _asplayer_controller (cast `PlayerController` (`self.GetController`)))
  (`EnhancedInputSubsystemInterface.AddMappingContext` (pcsubsystem `EnhancedInputLocalPlayerSubsystem` _asplayer_controller) "/Game/Input/IMC_PlayerControls.IMC_PlayerControls" 0 (struct))
  (set `PlayerController.bShowMouseCursor` true (`GameplayStatics.GetPlayerController` 0)))

(event `EnhancedInput|/Game/Input/FireWeapon`
  (params (ActionValue :type Boolean) (ElapsedSeconds :type "Float (double-precision)") (TriggeredSeconds :type "Float (double-precision)") (InputAction :type "InputAction Object Reference" :default "/Game/Input/FireWeapon.FireWeapon"))
  (bind _returnvalue (`GameplayStatics.GetPlayerController` 0))
  (bind (_worldlocation _worlddirection) (`PlayerController.DeprojectMousePositionToWorld` _returnvalue))
  (:`Started`
    (bind _outhit (`KismetSystemLibrary.LineTraceSingle` :`Start` (`self.K2_GetActorLocation` (`Controller.K2_GetPawn` _returnvalue)) :`End` (+ _worldlocation (* _worlddirection 100000.0)) :`TraceChannel` "TraceTypeQuery1" :`DrawDebugType` "ForDuration" :`DrawTime` 2.5))
    (bind (_bblockinghit _binitialoverlap _time _distance _location) (`GameplayStatics.BreakHitResult` _outhit))
    (`AISense_Hearing.ReportNoiseEvent` _location 1.0 self 5000.0)
    (`GameplayStatics.PlaySoundAtLocation` "/Game/StarterContent/Audio/Explosion01.Explosion01" _location (struct) 1.0 1.0 0.0 null null null null)))

(fn `UserConstructionScript`)