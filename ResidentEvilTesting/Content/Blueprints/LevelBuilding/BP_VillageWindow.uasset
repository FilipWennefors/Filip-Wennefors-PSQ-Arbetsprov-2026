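; Interactable village window that the player can vault through from either side.
; When confirmed as the closest interactable, it briefly shows a prompt widget turned toward the camera.
; Interaction picks start and destination by the player's side, using downward traces from front and back markers plus a capsule-height offset.
; It then snaps the player to the start, sets a motion warp target and plays the vault montage.
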(event `self.ReceiveTick`
  (params (DeltaSeconds :type "Float (single-precision)"))
  (`|AIMoveTo` (`GameplayStatics.GetPlayerPawn` 0) (0.0 0.0 0.0) null))

(event `self.OnConfirmedClosestInteractable`
  (`SceneComponent.K2_SetWorldRotation` (`self.Widget`) (`KismetMathLibrary.FindLookAtRotation` (`SceneComponent.K2_GetComponentLocation` (`self.Widget`)) (`PlayerCameraManager.GetCameraLocation` (`GameplayStatics.GetPlayerCameraManager` 0))) false false)
  (`SceneComponent.SetVisibility` (`self.Widget`) true true)
  (`KismetSystemLibrary.RetriggerableDelay` 0.1)
  (`SceneComponent.SetVisibility` (`self.Widget`) false false))

(event `self.Interact`)

(event `self.StartInteraction`
  (bind _returnvalue (+ (`self.GetPlayerVaultOffset`) (`self.LeapStartPosition`)))
  (bind (_returnvalue_roll _returnvalue_pitch _returnvalue_yaw) (`KismetMathLibrary.BreakRotator` (`KismetMathLibrary.FindLookAtRotation` _returnvalue (`self.LeapDestinationPosition`))))
  (if (`GeneralUtilities.IsActorInFront` (`GameplayStatics.GetPlayerPawn` 0) self)
    (bind _location (`self.TryGetFrontPosition`))
    (set `self.LeapStartPosition` _location)
    (bind _location_2 (`self.TryGetBackPosition`))
    (set `self.LeapDestinationPosition` _location_2)
    (else
      (bind _location_3 (`self.TryGetBackPosition`))
      (set `self.LeapStartPosition` _location_3)
      (bind _location_4 (`self.TryGetFrontPosition`))
      (set `self.LeapDestinationPosition` _location_4)))
  (`self.K2_SetActorTransform` (`GameplayStatics.GetPlayerPawn` 0) (`KismetMathLibrary.MakeTransform` _returnvalue (`KismetMathLibrary.MakeRotator` 0.0 0.0 _returnvalue_yaw)) false false)
  (bind _asplayer_character (cast `PlayerCharacter` (`GameplayStatics.GetPlayerPawn` 0)))
  (`CustomMotionWarpComponent.SetMotionWarpTarget` (`PlayerCharacter.CustomMotionWarper` _asplayer_character) "LeapWarping" (`KismetMathLibrary.MakeTransform` (+ (`self.GetPlayerVaultOffset`) (`self.LeapDestinationPosition`)) (`SceneComponent.K2_GetComponentRotation` (`self.BackLeapThroughPos`))))
  (`PlayMontageOnPlayerWithCallbacks.PlayMontageOnPlayerWithCallbacks` (`Character.Mesh` _asplayer_character) "/Game/Animations/LeonCustomAnimations/Montages/Ue5Rig_Leon_VaultThroughWindow_Montage.Ue5Rig_Leon_VaultThroughWindow_Montage" 1.0))

(fn `CanInteractWithObject`
  (returns (ReturnValue :type Boolean))
  (return true))

(fn `GetPlayerVaultOffset`
  (returns (ReturnValue :type "Vector Structure"))
  (return (`KismetMathLibrary.MakeVector` 0.0 0.0 (.z (`.BoxExtent` (`self.GetActorBounds` (`GameplayStatics.GetPlayerPawn` 0) true false))))))

(fn `TryGetBackPosition`
  (returns (Location :type "Vector Structure"))
  (bind _backleapthroughpos (`self.BackLeapThroughPos`))
  (bind (_outhit _returnvalue) (`KismetSystemLibrary.LineTraceSingle` (`SceneComponent.K2_GetComponentLocation` (`self.BackLeapThroughPos`)) (+ (`SceneComponent.K2_GetComponentLocation` _backleapthroughpos) (* (`SceneComponent.GetUpVector` _backleapthroughpos) -100000.0)) "TraceTypeQuery1"))
  (if _returnvalue
    (return (`.Location` (`GameplayStatics.BreakHitResult` _outhit)))))

(fn `TryGetFrontPosition`
  (returns (Location :type "Vector Structure"))
  (bind _frontleapthroughpos (`self.FrontLeapThroughPos`))
  (bind (_outhit _returnvalue) (`KismetSystemLibrary.LineTraceSingle` (`SceneComponent.K2_GetComponentLocation` (`self.FrontLeapThroughPos`)) (+ (`SceneComponent.K2_GetComponentLocation` _frontleapthroughpos) (* (`SceneComponent.GetUpVector` _frontleapthroughpos) -100000.0)) "TraceTypeQuery1"))
  (if _returnvalue
    (return (`.Location` (`GameplayStatics.BreakHitResult` _outhit)))))

(fn `UserConstructionScript`)