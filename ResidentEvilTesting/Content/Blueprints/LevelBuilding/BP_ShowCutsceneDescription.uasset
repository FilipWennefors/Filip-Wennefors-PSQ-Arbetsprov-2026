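; Level trigger actor that shows timed descriptive cutscene text on screen when the player pawn overlaps it.
; On overlap it sets HasPlayedOnce, without checking it, and adds a WBP_CutsceneDescription widget to the viewport.
; A looping Delay steps through the DescriptionTextLines array at a fixed interval.
; After the last line it removes the widget and fires OnFinished.
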(event `self.ReceiveActorBeginOverlap`
  (params (OtherActor :type "Actor Object Reference"))
  (if (== OtherActor (`GameplayStatics.GetPlayerPawn` 0))
    (set `self.HasPlayedOnce` true)
    (bind _returnvalue (`|CreateWidget` "/Game/Blueprints/WidgetBlueprints/WBP_CutsceneDescription.WBP_CutsceneDescription_C" (`GameplayStatics.GetPlayerController` 0)))
    (`UserWidget.AddToViewport` _returnvalue 0)
    (if (<= (`self.TextLine`) (- (`KismetArrayLibrary.Array_Length` (`self.Description Text Lines`)) 1)) :!label _label
      (`CutsceneDescription.SetDescriptiveText` _returnvalue (`|GetArrayItem` (`self.Description Text Lines`) (`self.TextLine`)))
      (set `self.TextLine` (+ (`self.TextLine`) 1))
      (`KismetSystemLibrary.Delay` 7.5)
      (goto _label)
      (else
        (`Widget.RemoveFromParent` _returnvalue)
        (`self.OnFinished`)))))

(fn `UserConstructionScript`)