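; BP_Door is an interactable hinged door that swings open and closed when StartInteraction is called.
; On opening, it checks whether the player pawn is in front and sets the swing direction accordingly.
; A Timeline drives the door's relative yaw, playing in reverse to close with the stored direction.
; CanOpenDoor blocks input during the swing, and the Timeline's finish toggles IsOpened and unlocks it.
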(event `self.StartInteraction`
  (bind _door (`self.Door`))
  (bind (_relativerotation_roll _relativerotation_pitch) (`KismetMathLibrary.BreakRotator` (`SceneComponent.RelativeRotation` _door)))
  (if (`self.CanOpenDoor`)
    (set `self.CanOpenDoor` false)
    (if (not (`self.IsOpened`))
      (if (`GeneralUtilities.IsActorInFront` (`GameplayStatics.GetPlayerPawn` 0) self)
        (set `self.RotationDirection` -1.0)
        (bind (_direction _doorrotation) (`Timeline|Timeline` :!via `PlayFromStart` :!label _label)
          (:`Update`
            (`SceneComponent.K2_SetRelativeRotation` _door (`KismetMathLibrary.MakeRotator` _relativerotation_roll _relativerotation_pitch (* _doorrotation (`self.RotationDirection`))) false false))
          (:`Finished`
            (set `self.IsOpened` (not (`self.IsOpened`)))
            (set `self.CanOpenDoor` true)))
        (else
          (set `self.RotationDirection` 1.0)
          (goto _label :!via `PlayFromStart`)))
      (else
        (goto _label :!via `ReverseFromEnd`)))))

(fn `UserConstructionScript`)