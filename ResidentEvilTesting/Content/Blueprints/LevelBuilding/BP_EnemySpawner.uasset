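; Enemy spawner actor that creates a requested number of enemies at its own transform, only while it is off screen.
; SpawnEnemies picks a random class from the supplied array for each spawn, though its Length-1 random bound never selects the last entry.
; Each enemy spawns with an axe, adjusting for collisions, and valid spawns are passed to CallOnEnemySpawned.
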(event `self.ReceiveTick`
  (params (DeltaSeconds :type "Float (single-precision)")))

(event `Spawn Enemies`
  (params (`Enemy Count` :type Integer) (`Enemy Classes` :type "Array of BaseEnemy Class Reference"))
  (bind _returnvalue (`self.IsEnemySpawnerOnScreen`))
  (if (not _returnvalue)
    (for _ (range 1 (+ `Enemy Count` 1))
      (bind _returnvalue_2 (`|SpawnActorFromClass` (`|GetArrayItem` `Enemy Classes` (`KismetMathLibrary.RandomInteger` (- (`KismetArrayLibrary.Array_Length` `Enemy Classes`) 1))) (`self.GetTransform`) "AdjustIfPossibleButAlwaysSpawn" "OverrideRootScale" null "/Game/WeaponClasses/EnemyWeapons/BP_Axe.BP_Axe_C" null))
      (if (`KismetSystemLibrary.IsValid` _returnvalue_2)
        (`self.OnEnemySpawned` _returnvalue_2)
        (else
          (`KismetSystemLibrary.PrintString` "Spawnactor returned null"))))
    (`KismetSystemLibrary.PrintString` "Spawned Enemies")))

(fn `UserConstructionScript`)