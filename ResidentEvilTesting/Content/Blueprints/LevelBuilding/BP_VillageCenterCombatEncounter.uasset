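; Village center combat encounter that keeps the fight populated, then ends it with a church bell and the end-of-game screen.
; Each kill checks the enemy count and, below the minimum, spawns more from the off-screen spawner closest to the player.
; The first kill starts the encounter timer.
; On expiry, the bell rings, enemies run a walk-to-church behavior tree, and a text cutscene leads to a paused thanks-for-playing widget.
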(event `self.OnEnemyKilled`
  (params (enemyKilled :type "BaseEnemy Object Reference") (bIsReallyDead :type Boolean))
  (`KismetSystemLibrary.PrintString` (`KismetStringLibrary.BuildString_Name` "Killed Enemy: " "" (`KismetStringLibrary.Conv_StringToName` (`KismetSystemLibrary.GetObjectName` enemyKilled))))
  (`|ExecutionSequence`
    (:`then_0`
      (if (not (`self.HasKilledFirstEnemy`))
        (set `self.HasKilledFirstEnemy` true)
        (`self.OnFirstEnemyKilled`)))
    (:`then_1`
      (`self.Check If Enough Enemies`))))

(event `OnFirstEnemyKilled`
  (`KismetSystemLibrary.Delay` (`self.EncounterDuration`))
  (`/Game/Blueprints/LevelBuilding/BP_SoundEmitter.PlaySoundEffect` (`self.BellSoundEmitter`))
  (`|ExecutionSequence`
    (:`then_0`
      ;[0 0 0] Show Cutscene Description
      (`KismetSystemLibrary.Delay` 5.0)
      (bind _returnvalue (`|SpawnActorFromClass` "/Game/Blueprints/LevelBuilding/BP_ShowCutsceneDescription.BP_ShowCutsceneDescription_C" (`self.GetTransform` (`GameplayStatics.GetPlayerPawn` 0)) "AlwaysSpawn" "OverrideRootScale" null (`|MakeArray` "The villagers slowly start walking towards the church. One of them drops their axe on the ground" "Leon looks at the villagers behaviour confused. After the final villager has entered the church, he closes and locks the door behind him." "Overlooking the now empty battlefield, Leon sarcastically remarks \"Where is everyone going? Bingo?\"") null))
      (add `/Game/Blueprints/LevelBuilding/BP_ShowCutsceneDescription.OnFinished` _returnvalue (delegate `OnFinished`)))
    (:`then_1`
      ;[0 0 0] Makes all enemies walk towards the church
      (for _array_element (`self.encounterEnemies`)
        (if (`KismetSystemLibrary.IsValid` _array_element)
          (bind _asbase_enemy_controller (cast `BaseEnemyController` (`Pawn.GetController` _array_element)))
          (`BaseEnemyController.RunPreScriptedBehaviour` _asbase_enemy_controller "/Game/Blueprints/EnemyAI/BT_WalkTowardsChurch.BT_WalkTowardsChurch")
          (`BlackboardComponent.SetValueAsVector` (`AIBlueprintHelperLibrary.GetBlackboard` _asbase_enemy_controller) "ChurchPosition" (`self.K2_GetActorLocation` (`self.Church`))))))))

(event `OnFinished`
  ;[0 0 0] Show Thanks for playing message
  (bind _returnvalue (`|CreateWidget` "/Game/Blueprints/WidgetBlueprints/WBP_ThanksForPlaying.WBP_ThanksForPlaying_C" (`GameplayStatics.GetPlayerController` 0)))
  (`UserWidget.AddToViewport` _returnvalue 0)
  (set `PlayerController.bShowMouseCursor` true (`GameplayStatics.GetPlayerController` 0))
  (`WidgetBlueprintLibrary.SetInputMode_GameAndUIEx` (`GameplayStatics.GetPlayerController` 0) _returnvalue)
  (`GameplayStatics.SetGamePaused` true))

(event `self.ReceiveTick`
  (params (DeltaSeconds :type "Float (single-precision)"))
  (`KismetSystemLibrary.PrintString` (`KismetStringLibrary.BuildString_Int` "Amount of enemies is" "" (`self.enemiesCount`)) true true (struct :`G` 0.66 :`B` 1.0 :`A` 1.0) 2.0 "EnemiesCount"))

(event `Check If Enough Enemies`
  (if (< (`self.enemiesCount`) (`self.MinEnemiesCount`))
    (bind _bestenemyspawner (`self.FindBestEnemySpawner`))
    (`/Game/Blueprints/LevelBuilding/BP_EnemySpawner.Spawn Enemies` _bestenemyspawner (- (`self.MaxEnemiesCount`) (`self.MinEnemiesCount`)) (`|MakeArray` "/Game/Blueprints/EnemyAI/BP_AttackingEnemyTest.BP_AttackingEnemyTest_C" :!type "BaseEnemy Class Reference"))))

(fn `FindBestEnemySpawner`
  (returns (BestEnemySpawner :type "/Game/Blueprints/LevelBuilding/BP_EnemySpawner Object Reference"))
  (locals (EnemySpawnersNotOnScreen :type "Array of EnemySpawner Object Reference"))
  (`KismetArrayLibrary.Array_Clear` (`local.EnemySpawnersNotOnScreen`))
  (for _array_element (`self.EnemySpawners`)
    (bind _returnvalue (`EnemySpawner.IsEnemySpawnerOnScreen` _array_element))
    (if (not _returnvalue)
      (`KismetArrayLibrary.Array_Add` (`local.EnemySpawnersNotOnScreen`) _array_element)))
  (bind _asbp_enemy_spawner (cast `/Game/Blueprints/LevelBuilding/BP_EnemySpawner` (`GeneralUtilities.FindClosestActor` (`local.EnemySpawnersNotOnScreen`) (`self.K2_GetActorLocation` (`GameplayStatics.GetPlayerPawn` 0)))))
  (return _asbp_enemy_spawner))

(fn `UserConstructionScript`
  (bind _visualizationbox (`self.VisualizationBox`))
  (set `VisualizationBox.boxDimensions` (`self.boxSize`) _visualizationbox)
  (set `VisualizationBox.boxOffset` (`self.boxOffset`) _visualizationbox))