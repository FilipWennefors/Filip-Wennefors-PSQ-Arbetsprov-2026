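; BP_LockedDoor is an interactable door that stays locked until the required key is used on it.
; Interacting while locked opens WBP_UnlockDoorMenu linked to this door, pauses the game and shows the cursor; once unlocked, interaction defers to the parent.
; TryUseKey compares the supplied object's class to KeyRequired, and a match closes the menu and unlocks the door.
; Closing the menu restores game-only input and unpauses.
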(event `self.ReceiveBeginPlay`
  (`parent.ReceiveBeginPlay`)
  (set `self.CanOpenDoor` false))

(event `self.StartInteraction`
  (if (not (`self.CanOpenDoor`))
    (bind _returnvalue (`|CreateWidget` "/Game/Blueprints/WidgetBlueprints/WBP_UnlockDoorMenu.WBP_UnlockDoorMenu_C" (`GameplayStatics.GetPlayerController` 0) self))
    (`UserWidget.AddToViewport` _returnvalue 0)
    (set `self.UnlockMenu` _returnvalue)
    (`WidgetBlueprintLibrary.SetInputMode_GameAndUIEx` (`GameplayStatics.GetPlayerController` 0) (`self.UnlockMenu`))
    (set `PlayerController.bShowMouseCursor` true (`GameplayStatics.GetPlayerController` 0))
    (`GameplayStatics.SetGamePaused` true)
    (add `/Game/Blueprints/WidgetBlueprints/WBP_UnlockDoorMenu.OnMenuClosed` (`self.UnlockMenu`) (delegate `OnMenuClosed`))
    (else
      (`parent.StartInteraction`))))

(event `OnMenuClosed`
  (bind _returnvalue (`GameplayStatics.GetPlayerController` 0))
  (`Widget.RemoveFromParent` (`self.UnlockMenu`))
  (`WidgetBlueprintLibrary.SetInputMode_GameOnly` _returnvalue)
  (set `PlayerController.bShowMouseCursor` false _returnvalue)
  (`GameplayStatics.SetGamePaused` false))

(fn `TryUseKey`
  (params (Object :type "KeyItem Object Reference"))
  (if (== (`GameplayStatics.GetObjectClass` Object) (`self.KeyRequired`))
    (`self.OnMenuClosed`)
    (set `self.CanOpenDoor` true)))

(fn `UserConstructionScript`
  (`parent.UserConstructionScript`))