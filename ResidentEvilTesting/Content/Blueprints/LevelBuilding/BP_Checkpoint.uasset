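; Checkpoint actor that records itself with the game mode as the latest checkpoint when the player reaches it.
; Its Box overlap checks for player pawn 0, casts to BP_ResidentEvilGameMode and calls SetLatestCheckpoint, with debug prints along each branch.
; Instances flagged IsDefaultSpawnPoint also register from the construction script, which casts to ResidentEvilGameMode rather than the BP_ class used on overlap.
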(event `self.Box.OnComponentBeginOverlap`
  (params (OverlappedComponent :type "PrimitiveComponent Object Reference") (OtherActor :type "Actor Object Reference") (OtherComp :type "PrimitiveComponent Object Reference") (OtherBodyIndex :type Integer) (bFromSweep :type Boolean) (SweepResult :type "HitResult Structure (by ref)"))
  (`KismetSystemLibrary.PrintString` "On component begin overlap")
  (if (== OtherActor (`GameplayStatics.GetPlayerPawn` 0))
    (`KismetSystemLibrary.PrintString` "Overlapped player")
    (bind _asbp_resident_evil_game_mode (cast `/Game/Blueprints/BP_ResidentEvilGameMode` (`GameplayStatics.GetGameMode`))
      (:`then`
        (`ResidentEvilGameMode.SetLatestCheckpoint` _asbp_resident_evil_game_mode self))
      (:`CastFailed`
        (`KismetSystemLibrary.PrintString` "Cast failed")))
    (else
      (`KismetSystemLibrary.PrintString` "Did not overlap player"))))

(fn `UserConstructionScript`
  (if (`self.IsDefaultSpawnPoint`)
    (bind _asresident_evil_game_mode (cast `ResidentEvilGameMode` (`GameplayStatics.GetGameMode`)))
    (`ResidentEvilGameMode.SetLatestCheckpoint` _asresident_evil_game_mode self)))