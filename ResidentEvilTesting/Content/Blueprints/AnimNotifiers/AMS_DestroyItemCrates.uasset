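; Anim notify state that breaks item crates around the player character when its animation window begins.
; It runs a multi-sphere trace at the owning PlayerCharacter's location, ignoring the player and the equipped weapon and knife.
; Hit actors that cast to ItemCrate receive heavy damage through ApplyDamage.
; All work happens once in NotifyBegin, with no tick or end logic.
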(fn `Received_NotifyBegin`
  (params (MeshComp :type "SkeletalMeshComponent Object Reference") (Animation :type "AnimSequenceBase Object Reference") (TotalDuration :type "Float (single-precision)") (EventReference :type "AnimNotifyEventReference Structure (by ref)"))
  (returns (ReturnValue :type Boolean))
  (bind _asplayer_character (cast `PlayerCharacter` (`ActorComponent.GetOwner` MeshComp)))
  (bind _returnvalue (`Actor.K2_GetActorLocation` _asplayer_character))
  (bind (_outhits _returnvalue_2) (`KismetSystemLibrary.SphereTraceMulti` _asplayer_character _returnvalue _returnvalue 350.0 "TraceTypeQuery3" false (`|MakeArray` _asplayer_character (`PlayerCharacter.currentlyEquippedWeapon` _asplayer_character) (`PlayerCharacter.currentlyEquippedKnife` _asplayer_character) :!type "Actor Object Reference")))
  (if _returnvalue_2
    (for _array_element _outhits
      (bind _asitem_crate (cast `ItemCrate` (`.HitActor` (`GameplayStatics.BreakHitResult` _array_element))))
      (`GameplayStatics.ApplyDamage` _asitem_crate 1000.0))
    (return true)
    (else
      (return false))))