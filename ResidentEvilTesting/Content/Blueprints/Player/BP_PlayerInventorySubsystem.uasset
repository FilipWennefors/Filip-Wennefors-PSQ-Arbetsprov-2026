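; Player inventory subsystem for a grid inventory where items span several slots and can be rotated.
; On init it fills a flat slot array from the inventory size; add and move update item position, slot occupancy and fire an item-added call.
; Fit checks test an item's footprint, ignoring cells it already occupies.
; Footprint, marking and clearing helpers are defined outside this graph, and slots also store icon widgets.
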(event `self.OnInitializedBP`
  (bind (_returnvalue_x _returnvalue_y) (`KismetMathLibrary.BreakVector2D` (`self.GetInventorySize`)))
  (for _ (range 1 (+ (`KismetMathLibrary.FTrunc` (* _returnvalue_x _returnvalue_y)) 1))
    (`KismetArrayLibrary.Array_Add` (`self.inventorySlots`) (make `InventorySlot` false))))

(event `self.TestAddItem`
  (params (itemSize :type "Vector2D Structure") (inventoryPosition :type "Vector2D Structure") (bIsRotated :type Boolean)))

(fn `AddItemToSlot`
  (params (InInt :type Integer) (InInt1 :type Integer) (InputPin :type "NewInventoryItem Object Reference"))
  (set `NewInventoryItem.ItemPosition` (`KismetMathLibrary.MakeVector2D` (`KismetMathLibrary.Conv_IntToDouble` InInt) (`KismetMathLibrary.Conv_IntToDouble` InInt1)) InputPin)
  (`self.MarkSlotsAsOccupied` InputPin (`NewInventoryItem.bIsRotated` InputPin))
  (`self.OnItemAdded` InputPin))

(fn `Check If Item Fits Slot BP`
  (params (ItemToCheck :type "NewInventoryItem Object Reference") (X :type Integer) (Y :type Integer))
  (returns (`Item Fits In Slot` :type Boolean))
  (bind _slotstomark (`self.GetSlotsToMark` (`NewInventoryItem.ItemSize` ItemToCheck) (`KismetMathLibrary.MakeVector2D` (`KismetMathLibrary.Conv_IntToDouble` X) (`KismetMathLibrary.Conv_IntToDouble` Y)) (`NewInventoryItem.bIsRotated` ItemToCheck)))
  (for _array_element _slotstomark
    (bind (_bisoccupied _iteminslot) (break `InventorySlot` (`|GetArrayItem` (`self.inventorySlots`) _array_element)))
    (if _bisoccupied
      (if (not (`KismetMathLibrary.EqualExactly_Vector2DVector2D` (`NewInventoryItem.ItemPosition` _iteminslot) (`NewInventoryItem.ItemPosition` ItemToCheck)))
        (return false))))
  (return true))

(fn `CheckIfItemFitsInSlotWithBooleanParam`
  (params (IemToAdd :type "NewInventoryItem Object Reference") (X :type Integer) (Y :type Integer) (bIsRotated :type Boolean))
  (returns (`Item Fits In Slot` :type Boolean))
  (bind _returnvalue (`self.CheckIfItemFitsSlot` (`KismetMathLibrary.MakeVector2D` (`KismetMathLibrary.Conv_IntToDouble` X) (`KismetMathLibrary.Conv_IntToDouble` Y)) (`NewInventoryItem.ItemSize` IemToAdd) bIsRotated IemToAdd))
  (if _returnvalue
    (bind _slotstomark (`self.GetSlotsToMark` (`NewInventoryItem.ItemSize` IemToAdd) (`KismetMathLibrary.MakeVector2D` (`KismetMathLibrary.Conv_IntToDouble` X) (`KismetMathLibrary.Conv_IntToDouble` Y)) bIsRotated))
    (for _array_element _slotstomark
      (bind (_bisoccupied _iteminslot) (break `InventorySlot` (`|GetArrayItem` (`self.inventorySlots`) _array_element)))
      (if _bisoccupied
        (if (not (== _iteminslot IemToAdd))
          (return false))))
    (return true)
    (else
      (return false))))

(fn `Get Inventory Slots`
  (returns (InventorySlots :type "Array of InventorySlot Structure"))
  (return (`self.inventorySlots`)))

(fn `MoveItemToOtherSlot`
  (params (`Item To Move` :type "NewInventoryItem Object Reference") (`Was Item Previously Rotated` :type Boolean) (X :type Integer) (Y :type Integer))
  (locals (PriorPosition :type "Vector2D Structure"))
  (set `local.PriorPosition` (`NewInventoryItem.ItemPosition` `Item To Move`))
  (`self.ClearInventorySlots` (`NewInventoryItem.ItemSize` `Item To Move`) (`local.PriorPosition`) `Was Item Previously Rotated`)
  (set `NewInventoryItem.ItemPosition` (`KismetMathLibrary.MakeVector2D` (`KismetMathLibrary.Conv_IntToDouble` X) (`KismetMathLibrary.Conv_IntToDouble` Y)) `Item To Move`)
  (`self.MarkSlotsAsOccupied` `Item To Move` (`NewInventoryItem.bIsRotated` `Item To Move`))
  (`self.OnItemAdded` `Item To Move`))

(fn `SetImageIconInSlot`
  (params (Index :type Integer) (ImageWidget :type "ImageWidget Object Reference"))
  (setmembers `InventorySlot` :`StructRef` (`|GetArrayItem` (`self.inventorySlots`) Index) :`imageWidget` ImageWidget))