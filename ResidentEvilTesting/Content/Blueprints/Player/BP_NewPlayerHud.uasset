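; Player HUD Blueprint that creates the weapon wheel and in-game HUD at BeginPlay and manages menu screens.
; Toggle and show/hide functions drive the pause menu, tab-menu inventory and death screen, switching input mode and cursor visibility.
; The inventory widget is created once, then collapsed for reuse, and pauses the game while open.
; Item-added modals spawn from a supplied class with image and text, also pausing the game.
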(event `self.ReceiveBeginPlay`
  (bind _returnvalue (`GameplayStatics.GetPlayerController` 0))
  (bind _returnvalue_2 (`|CreateWidget` "/Game/Blueprints/WidgetBlueprints/WBP_WeaponWheel.WBP_WeaponWheel_C" _returnvalue))
  (`UserWidget.AddToViewport` _returnvalue_2 0)
  (bind _returnvalue_3 (`|CreateWidget` "/Game/Blueprints/WidgetBlueprints/WBP_InGameHudV2.WBP_InGameHudV2_C" _returnvalue))
  (`UserWidget.AddToViewport` _returnvalue_3 10))

(fn `DisableInventory`
  (`Widget.SetVisibility` (`self.PlayerInventoryReference`) "Collapsed")
  (`WidgetBlueprintLibrary.SetInputMode_GameOnly` (`GameplayStatics.GetPlayerController` 0))
  (set `PlayerController.bShowMouseCursor` false (`GameplayStatics.GetPlayerController` 0))
  (set `self.Is In inventory` false)
  (`GameplayStatics.SetGamePaused` false))

(fn `EnableInventory`
  (if (not (`KismetSystemLibrary.IsValid` (`self.PlayerInventoryReference`)))
    (bind _returnvalue (`|CreateWidget` "/Game/Blueprints/WidgetBlueprints/WBP_TabMenuManager.WBP_TabMenuManager_C" (`GameplayStatics.GetPlayerController` 0)))
    (bind _output_get (set `self.PlayerInventoryReference` _returnvalue))
    (`UserWidget.AddToViewport` _output_get 0)
    (else
      (`Widget.SetVisibility` (`self.PlayerInventoryReference`) "Visible")))
  (`WidgetBlueprintLibrary.SetInputMode_GameAndUIEx` (`GameplayStatics.GetPlayerController` 0) (`self.PlayerInventoryReference`) "DoNotLock" false) ; WARNING: HIDE CURSOR DURING CAPTURE BREAKS INVENTORY: DO NOT USE
  (set `PlayerController.bShowMouseCursor` true (`GameplayStatics.GetPlayerController` 0))
  (set `self.Is In inventory` true)
  (`GameplayStatics.SetGamePaused` true)
  (`TabMenuManager.OnOpened` (`self.PlayerInventoryReference`)))

(fn `HideDeathScreen`
  (`Widget.RemoveFromParent` (`self.DeathScreenReference`))
  (`WidgetBlueprintLibrary.SetInputMode_GameOnly` (`GameplayStatics.GetPlayerController` 0))
  (set `PlayerController.bShowMouseCursor` false (`GameplayStatics.GetPlayerController` 0)))

(fn `HidePauseMenu`
  (`Widget.RemoveFromParent` (`self.PauseMenuReference`))
  (`WidgetBlueprintLibrary.SetInputMode_GameOnly` (`GameplayStatics.GetPlayerController` 0))
  (set `PlayerController.bShowMouseCursor` false (`GameplayStatics.GetPlayerController` 0)))

(fn `Show Item Added Modal`
  (params (ModalClass :type "/Game/Blueprints/WidgetBlueprints/WBP_ItemAddedModal Class Reference") (modalImageTexture :type "Texture2D Object Reference") (modalTextBig :type String) (modalTextSmaller :type String))
  (bind _returnvalue (`|CreateWidget` ModalClass (`GameplayStatics.GetPlayerController` 0) modalImageTexture modalTextBig modalTextSmaller))
  (`UserWidget.AddToViewport` _returnvalue 11)
  (`WidgetBlueprintLibrary.SetInputMode_GameAndUIEx` (`GameplayStatics.GetPlayerController` 0) _returnvalue)
  (set `PlayerController.bShowMouseCursor` true (`GameplayStatics.GetPlayerController` 0))
  (`GameplayStatics.SetGamePaused` true))

(fn `ShowDeathScreen`
  (bind _returnvalue (`GameplayStatics.GetPlayerController` 0))
  (bind _returnvalue_2 (`|GenericCreateObject` _returnvalue "/Game/Blueprints/WidgetBlueprints/WBP_DeathScreen.WBP_DeathScreen_C"))
  (bind _output_get (set `self.DeathScreenReference` _returnvalue_2))
  (`UserWidget.AddToViewport` _output_get 11)
  (`WidgetBlueprintLibrary.SetInputMode_UIOnlyEx` _returnvalue _output_get)
  (set `PlayerController.bShowMouseCursor` true _returnvalue))

(fn `ShowPauseMenu`
  (bind _returnvalue (`|GenericCreateObject` (`GameplayStatics.GetPlayerController` 0) "/Game/Blueprints/WidgetBlueprints/WBP_PauseMenu.WBP_PauseMenu_C"))
  (`UserWidget.AddToViewport` _returnvalue 0)
  (set `self.PauseMenuReference` _returnvalue)
  (`WidgetBlueprintLibrary.SetInputMode_GameAndUIEx` (`GameplayStatics.GetPlayerController` 0) (`self.PauseMenuReference`))
  (set `PlayerController.bShowMouseCursor` true (`GameplayStatics.GetPlayerController` 0)))

(fn `ToggleInventory`
  (if (not (`self.Is In inventory`))
    (`self.EnableInventory`)
    (else
      (`self.DisableInventory`))))

(fn `TogglePauseMenu`
  (returns (UpdatedPauseState :type Boolean))
  (if (not (`GameplayStatics.IsGamePaused`))
    (`self.ShowPauseMenu`)
    (return true)
    (elif (not (`self.Is In inventory`))
      (`self.HidePauseMenu`)
      (return false))))

(fn `UserConstructionScript`)