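; Game mode for a Resident Evil-style game that handles player spawning and checkpoint respawns.
; FindPlayerStart returns the latest recorded checkpoint if valid, otherwise defers to ChoosePlayerStart.
; That fallback prefers an enabled default BP_Checkpoint, else takes the first candidate among enabled checkpoints and plain PlayerStarts.
; RestartfromCheckpoint destroys the player pawn and restarts the player after a brief delay.
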(event `self.RestartFromCheckpoint`
  (`self.K2_DestroyActor` (`GameplayStatics.GetPlayerPawn` 0))
  (`KismetSystemLibrary.Delay` 0.2)
  (`self.RestartPlayer` (`GameplayStatics.GetPlayerController` 0)))

(event `self.SetLatestCheckpoint`
  (params (latestCheckpoint :type "Checkpoint Object Reference"))
  (bind _output_get (set `self.Latest Checkpoint` latestCheckpoint))
  (`KismetSystemLibrary.PrintString` (`KismetStringLibrary.BuildString_Name` "Set latest checkpoint to" "" (`KismetStringLibrary.Conv_StringToName` (`KismetSystemLibrary.GetObjectName` _output_get)))))

(fn `ChoosePlayerStart_BP`
  (params (playerController :type "Controller Object Reference"))
  (returns (ReturnValue :type "Actor Object Reference"))
  (locals (PossiblePlayerStarts :type "Array of Actor Object Reference"))
  (bind _outactors (`GameplayStatics.GetAllActorsOfClass` "/Script/Engine.PlayerStart"))
  (for _array_element _outactors
    (bind _asbp_checkpoint (cast `/Game/Blueprints/LevelBuilding/BP_Checkpoint` _array_element)
      (:`then`
        (if (`/Game/Blueprints/LevelBuilding/BP_Checkpoint.IsEnabled` _asbp_checkpoint)
          (if (`/Game/Blueprints/LevelBuilding/BP_Checkpoint.IsDefaultSpawnPoint` _asbp_checkpoint)
            (return _asbp_checkpoint)
            (else
              (`KismetArrayLibrary.Array_Add` (`local.PossiblePlayerStarts`) _asbp_checkpoint)))))
      (:`CastFailed`
        (`KismetArrayLibrary.Array_Add` (`local.PossiblePlayerStarts`) _array_element))))
  (for _array_element_2 (`local.PossiblePlayerStarts`)
    (return _array_element_2)))

(fn `FindPlayerStart`
  (params (Player :type "Controller Object Reference") (IncomingName :type String))
  (returns (ReturnValue :type "Actor Object Reference"))
  (bind _latest_checkpoint (`self.Latest Checkpoint`))
  (if (`KismetSystemLibrary.IsValid` _latest_checkpoint)
    (return _latest_checkpoint)
    (else
      (bind _returnvalue (`self.ChoosePlayerStart_BP` Player))
      (return _returnvalue))))

(fn `UserConstructionScript`)