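; BP_TestEnemy is an experimental AI enemy character that can be staggered.
; On BeginPlay it applies its walk speed and binds to stagger changes from BPCDamagableEnemyComponent.
; Stagger disables movement and recovery restores walking, with the state mirrored to the IsStaggered Blackboard key.
; The construction script registers both knees and the head as the component's weak points.
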(event `self.ReceiveBeginPlay`
  (set `CharacterMovementComponent.MaxWalkSpeed` (`self.WalkSpeed`) (`self.CharacterMovement`))
  (add `/Game/Blueprints/EnemyAI/BPC_DamagableEnemyComponent.OnStaggerChanged` (`self.BPC_DamagableEnemyComponent`) (delegate `CustomEvent`)))

(event `CustomEvent`
  (params (IsStaggered :type Boolean))
  (if IsStaggered
    (`CharacterMovementComponent.DisableMovement` (`self.CharacterMovement`))
    (else
      (`CharacterMovementComponent.SetMovementMode` (`self.CharacterMovement`) "MOVE_Walking" 0)))
  (`BlackboardComponent.SetValueAsBool` (`AIBlueprintHelperLibrary.GetBlackboard` (`AIBlueprintHelperLibrary.GetAIController` self)) "IsStaggered" IsStaggered))

(event `self.ReceiveTick`
  (params (DeltaSeconds :type "Float (single-precision)")))

(event `self.ReceivePointDamage`
  (params (Damage :type "Float (single-precision)") (DamageType :type "DamageType Object Reference") (HitLocation :type "Vector Structure") (HitNormal :type "Vector Structure") (HitComponent :type "PrimitiveComponent Object Reference") (BoneName :type Name) (ShotFromDirection :type "Vector Structure") (InstigatedBy :type "Controller Object Reference") (DamageCauser :type "Actor Object Reference") (HitInfo :type "HitResult Structure (by ref)")))

(fn `UserConstructionScript`
  (set `DamagableEnemyComponent.weakPoints` (`|MakeArray` (`self.Knee_R`) (`self.Knee_L`) (`self.Head`) :!type "ShapeComponent Object Reference") (`self.BPC_DamagableEnemyComponent`)))