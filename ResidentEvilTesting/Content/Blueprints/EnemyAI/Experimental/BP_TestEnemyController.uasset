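; Experimental AI controller for test enemies that tracks the player through AI Perception.
; On BeginPlay it runs the BT_EnemyBehaviour behavior tree.
; When perception updates for the player pawn, it writes the stimulus location to LastKnownPlayerLocation and the sensed state to CanSeePlayer on the blackboard.
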(event `self.ReceiveBeginPlay`
  (`self.RunBehaviorTree` "/Game/Blueprints/EnemyAI/Experimental/BT_EnemyBehaviour.BT_EnemyBehaviour"))

(event `self.ReceiveTick`
  (params (DeltaSeconds :type "Float (single-precision)")))

(event `self.AIPerception.OnTargetPerceptionUpdated`
  (params (Actor :type "Actor Object Reference") (Stimulus :type "AIStimulus Structure"))
  (bind (_age _expirationage _strength _stimuluslocation _receiverlocation _tag _bsuccessfullysensed) (break `AIStimulus` Stimulus))
  (if (== Actor (`GameplayStatics.GetPlayerPawn` 0))
    (`BlackboardComponent.SetValueAsVector` (`AIBlueprintHelperLibrary.GetBlackboard` null) "LastKnownPlayerLocation" _stimuluslocation)
    (`BlackboardComponent.SetValueAsBool` (`AIBlueprintHelperLibrary.GetBlackboard` null) "CanSeePlayer" _bsuccessfullysensed)))

(fn `UserConstructionScript`)