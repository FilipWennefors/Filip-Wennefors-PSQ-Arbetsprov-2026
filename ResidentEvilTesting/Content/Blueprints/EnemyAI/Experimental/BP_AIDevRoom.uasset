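; Experimental enemy character that attacks with a socket-attached weapon, reacts to hits and ragdolls on death.
; Point damage reads per-component collision params, playing a duration-scaled hit montage with stun on normal areas.
; Weak-spot hits accumulate stagger damage, which past a threshold rolls a stagger chance and picks an animation by component name.
; Parried attacks stagger directly, and the kill function pauses montages, enables mesh physics and disables capsule collision.
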(event `self.ReceiveBeginPlay`
  (bind _weaponmesh (`EnemyBaseWeapon.weaponMesh` (`self.equippedWeaponActor`)))
  ;[0 0 0] Attach Weapon To Enemy
  (if (`KismetSystemLibrary.IsValidClass` (`self.EquippedWeapon`))
    (bind _returnvalue (`|SpawnActorFromClass` (`self.EquippedWeapon`) (`SceneComponent.GetSocketTransform` (`self.Mesh`) "weapon_r" "RTS_World") "Undefined" "OverrideRootScale" null null))
    (bind _output_get (set `self.equippedWeaponActor` _returnvalue))
    (`self.K2_AttachToComponent` _output_get (`self.Mesh`) "weaponSocket_r" "SnapToTarget" "SnapToTarget" "SnapToTarget" true)
    (`SceneComponent.K2_SetRelativeTransform` _weaponmesh (`KismetMathLibrary.InvertTransform` (`SceneComponent.GetSocketTransform` _weaponmesh "Socket.Offset" "RTS_Component")) false false)))

(event `self.OnHitActor`
  (params (hitActor :type "Actor Object Reference"))
  ;[0 0 0] Called when the enemy hits a actor with an attack to damage the actor
  (`GameplayStatics.ApplyDamage` hitActor 50.0 null self))

(event `self.ReceivePointDamage`
  (params (Damage :type "Float (single-precision)") (DamageType :type "DamageType Object Reference") (HitLocation :type "Vector Structure") (HitNormal :type "Vector Structure") (HitComponent :type "PrimitiveComponent Object Reference") (BoneName :type Name) (ShotFromDirection :type "Vector Structure") (InstigatedBy :type "Controller Object Reference") (DamageCauser :type "Actor Object Reference") (HitInfo :type "HitResult Structure (by ref)"))
  (bind _output_get (set `self.Hit Component` HitComponent))
  (bind _collisioncompparams (message `EnemyHitComponent.GetCollisionCompParams` _output_get))
  (set `self.OnHitMontage` (break `EnemyCollisionCompParams` _collisioncompparams))
  (set `self.HitStunDuration` (`.hitStunDuration` (break `EnemyCollisionCompParams` _collisioncompparams)))
  (if (not (`.bIsWeakSpot` (break `EnemyCollisionCompParams` _collisioncompparams)))
    (`self.PlayAnimMontage` (`self.OnHitMontage`) (/ 1.0 (`self.HitStunDuration`)))
    (`self.ApplyStunEffect` (`self.HitStunDuration`))
    (`KismetSystemLibrary.PrintString` (`KismetStringLibrary.BuildString_Name` "Hit Component " "" (`KismetStringLibrary.Conv_StringToName` (`KismetSystemLibrary.GetObjectName` (`self.Hit Component`)))))
    (else
      (`self.ApplyStaggerDamage` Damage (`self.Hit Component`)))))

(event `self.NotifyOnAttackParried`
  (`self.StaggerEnemy` null (`self.StaggerDuration`) "/Game/Animations/GanadoCustomAnimations/Montages/Ue5Rig_Ganado_MeleeParryStagger_Montage.Ue5Rig_Ganado_MeleeParryStagger_Montage"))

(fn `ApplyStaggerDamage`
  (params (`Base Damage Taken` :type "Float (double-precision)") (`Hit Component` :type "PrimitiveComponent Object Reference"))
  (locals (DamageAboveTreshold :type "Float (double-precision)") (MaxDamageAboveThreshold :type "Float (double-precision)") (DamageAboveThresholdFactor :type "Float (double-precision)" :default 0.0) (`Remaning factor` :type "Float (double-precision)") (FactorToGuaranteedStagger :type "Float (double-precision)" :default 0.0))
  (bind (_value _returnvalue) (`BlueprintMapLibrary.Map_Find` (`self.Stagger Response Anims`) (`KismetStringLibrary.Conv_StringToName` (`KismetSystemLibrary.GetObjectName` `Hit Component`))))
  ;[0 0 0] If the Damage is below the threshold, don't apply stagger damage
  (bind _output_get (set `self.Stagger Damage dealt` (+ (`self.Stagger Damage dealt`) `Base Damage Taken`)))
  (if (>= _output_get (`self.Min Damage Stagger Threshold`))
    (bind _returnvalue_2 (`self.CalculateStaggerChance` (`self.Stagger Damage dealt`) (`self.Min Damage Stagger Threshold`) (`self.Guaranteed Stagger Damage Threshold`) (`self.Min Stagger chance`)))
    (if (and (>= _returnvalue_2 (`KismetMathLibrary.RandomFloatInRange` 0.0 100.0)) _returnvalue)
      (`self.StaggerEnemy` `Hit Component` (`self.StaggerDuration`) _value))))

(fn `BP Kill Enemy`
  (`AnimInstance.Montage_Pause` (`SkeletalMeshComponent.GetAnimInstance` (`self.Mesh`)) null)
  (`PrimitiveComponent.SetSimulatePhysics` (`self.Mesh`) true)
  (`self.SetCollisionResponseToRagdoll`)
  (`PrimitiveComponent.SetCollisionEnabled` (`self.CapsuleComponent`) "NoCollision"))

(fn `SetCollisionChannelsForRagdolls`
  (params (Target :type "PrimitiveComponent Object Reference"))
  (`PrimitiveComponent.SetCollisionResponseToChannel` Target "ECC_Visibility" "ECR_Ignore")
  (`PrimitiveComponent.SetCollisionResponseToChannel` Target "ECC_Camera" "ECR_Block")
  (`PrimitiveComponent.SetCollisionResponseToChannel` Target "ECC_GameTraceChannel1" "ECR_Overlap")
  (`PrimitiveComponent.SetCollisionResponseToChannel` Target "ECC_WorldStatic" "ECR_Block")
  (`PrimitiveComponent.SetCollisionResponseToChannel` Target "ECC_WorldDynamic" "ECR_Block")
  (`PrimitiveComponent.SetCollisionResponseToChannel` Target "ECC_Pawn" "ECR_Ignore")
  (`PrimitiveComponent.SetCollisionResponseToChannel` Target "ECC_PhysicsBody" "ECR_Block")
  (`PrimitiveComponent.SetCollisionResponseToChannel` Target "ECC_Vehicle" "ECR_Block")
  (`PrimitiveComponent.SetCollisionResponseToChannel` Target "ECC_Destructible" "ECR_Block"))

(fn `UserConstructionScript`
  (set `self.health` (`self.maxHealth`))
  (set `DamagableEnemyComponent.weakPoints` (`|MakeArray` null null null :!type "ShapeComponent Object Reference") (`self.BPC_DamagableEnemyComponent`)))