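; Experimental enemy test Blueprint for damage, weak points and stagger.
; Construction Script registers the head and both knees as weak points on DamagableEnemyComponent.
; CalculateStaggerChance accumulates damage and scales stagger chance linearly from its minimum toward 100 percent between the minimum-damage and guaranteed-stagger thresholds.
; PointDamage and CheckIfHitWeakSpot are empty, and nothing in the graphs calls the stagger calculation.
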(event `self.ReceiveBeginPlay`)

(event `self.ReceiveTick`
  (params (DeltaSeconds :type "Float (single-precision)")))

(event `self.ReceivePointDamage`
  (params (Damage :type "Float (single-precision)") (DamageType :type "DamageType Object Reference") (HitLocation :type "Vector Structure") (HitNormal :type "Vector Structure") (HitComponent :type "PrimitiveComponent Object Reference") (BoneName :type Name) (ShotFromDirection :type "Vector Structure") (InstigatedBy :type "Controller Object Reference") (DamageCauser :type "Actor Object Reference") (HitInfo :type "HitResult Structure (by ref)")))

(fn `CalculateStaggerChance`
  (returns (StaggerChance :type "Float (double-precision)"))
  (bind _output_get (set `self.DamageDealtForStaggerPurposes` (+ (`self.DamageDealtForStaggerPurposes`) (`self.DamageDealt`))))
  (bind _output_get_2 (set `self.AdditionalPercentToAdd` (- 1.0 (`KismetMathLibrary.FClamp` (/ (`self.MinStaggerChance`) 100.0)))))
  (return (+ (`self.MinStaggerChance`) (* (* (`KismetMathLibrary.FClamp` (/ (- _output_get (`self.MinDamageToStagger`)) (- (`self.WeakSpotDamageGuaranteedStaggerThreshold`) (`self.MinDamageToStagger`)))) _output_get_2) 100.0))))

(fn `CheckIfHitWeakSpot`
  (params (`Hit Component` :type "Object Object Reference")))

(fn `UserConstructionScript`
  (set `/Game/Blueprints/EnemyAI/BPC_DamagableEnemyComponent.weakPoints` (`|MakeArray` (`self.Head`) (`self.Knee_L`) (`self.Knee_R`) :!type "ShapeComponent Object Reference") (`self.DamagableEnemyComponent`)))