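; Test AI controller for an attacking enemy that runs BT_AttackingEnemyTree and feeds its blackboard from perception.
; Sight stores the player's position, clearing it on loss only if the stimulus has expired.
; Hearing stores a position to investigate, cleared after a retriggerable delay.
; Two functions support pre-scripted behaviour: one sets a blackboard object, while V2 injects a dynamic subtree by gameplay tag and raises a flag.
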(event `self.ReceiveBeginPlay`
  (`self.RunBehaviorTree` "/Game/Blueprints/EnemyAI/BT_AttackingEnemyTree.BT_AttackingEnemyTree"))

(event `self.OnTargetPerceptionUpdatedSight`
  (params (Actor :type "Actor Object Reference") (AIStimulus :type "AIStimulus Structure"))
  (bind _asplayer_character (cast `PlayerCharacter` Actor))
  (if AIStimulus_bSuccessfullySensed
    (`BlackboardComponent.SetValueAsVector` (`AIBlueprintHelperLibrary.GetBlackboard` (`AIBlueprintHelperLibrary.GetAIController` self)) "PlayerPosition" (`self.K2_GetActorLocation` _asplayer_character))
    (elif (>= AIStimulus_Age AIStimulus_ExpirationAge)
      (`BlackboardComponent.ClearValue` (`AIBlueprintHelperLibrary.GetBlackboard` (`AIBlueprintHelperLibrary.GetAIController` self)) "PlayerPosition"))))

(event `self.OnTargetPerceptionUpdatedHearing`
  (params (Actor :type "Actor Object Reference") (AIStimulus :type "AIStimulus Structure"))
  (if AIStimulus_bSuccessfullySensed
    (`BlackboardComponent.SetValueAsVector` (`AIBlueprintHelperLibrary.GetBlackboard` (`AIBlueprintHelperLibrary.GetAIController` self)) "PositionToInvestigate" AIStimulus_StimulusLocation)
    (`KismetSystemLibrary.RetriggerableDelay` 15.0)
    (`BlackboardComponent.ClearValue` (`AIBlueprintHelperLibrary.GetBlackboard` (`AIBlueprintHelperLibrary.GetAIController` self)) "PositionToInvestigate")))

(event `self.OnControlledEnemyKilled`)

(fn `Run Pre Scripted BehaviourBP`
  (params (ObjectValue :type "Object Object Reference"))
  (`BlackboardComponent.SetValueAsObject` (`AIBlueprintHelperLibrary.GetBlackboard` (`AIBlueprintHelperLibrary.GetAIController` self)) "PreScriptedBehaviour" ObjectValue))

(fn `RunPreScriptedBehaviourV2`
  (params (BehaviorAsset :type "BehaviorTree Object Reference"))
  (bind _asbehavior_tree_component (cast `BehaviorTreeComponent` (`self.BrainComponent`)))
  (`BehaviorTreeComponent.SetDynamicSubtree` _asbehavior_tree_component (struct :`TagName` "AttackingEnemy.ScriptedBehaviour") BehaviorAsset)
  (`BlackboardComponent.SetValueAsBool` (`AIBlueprintHelperLibrary.GetBlackboard` (`AIBlueprintHelperLibrary.GetAIController` self)) "ShouldRunPreScriptedBehavior" true))

(fn `UserConstructionScript`)