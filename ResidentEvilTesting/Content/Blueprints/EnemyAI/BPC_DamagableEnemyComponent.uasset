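; Enemy damage component that staggers its owner when point damage hits a weak-point shape.
; Unless already staggered, a weak-point hit rolls against CalculateStaggerChance, then plays a montage keyed by hit component name, rate-scaled by StaggerRecoverTime.
; Only montage completion clears the stagger; interruption just prints.
; BPCalculateStaggerChance maps accumulated damage to a chance above a minimum, but is not called here, and the damage-decay logic is disconnected.
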(event `self.ReceiveBeginPlay`)

(event `self.ReceiveTick`
  (params (DeltaSeconds :type "Float (single-precision)")))

(event `self.OnOwnerTakePointDamage`
  (params (DamagedActor :type "Actor Object Reference") (Damage :type "Float (single-precision)") (InstigatedBy :type "Controller Object Reference") (HitLocation :type "Vector Structure") (FHitComponent :type "PrimitiveComponent Object Reference") (BoneName :type Name) (ShotFromDirection :type "Vector Structure") (DamageType :type "DamageType Object Reference") (DamageCauser :type "Actor Object Reference"))
  (bind (_value _returnvalue) (`BlueprintMapLibrary.Map_Find` (`self.staggerAnimations`) (`KismetStringLibrary.Conv_StringToName` (`KismetSystemLibrary.GetObjectName` FHitComponent))))
  (set `self.damageDealt` Damage)
  (if (not (`self.isStaggered`))
    (bind _asshape_component (cast `ShapeComponent` FHitComponent))
    (bind _returnvalue_2 (`self.CheckIfHitComponentIsWeakPoint` _asshape_component))
    (if _returnvalue_2
      (bind _returnvalue_3 (`self.CalculateStaggerChance`))
      (if (>= _returnvalue_3 (`KismetMathLibrary.RandomFloatInRange` 0.0 100.0))
        (set `self.isStaggered` true)
        (set `self.staggerRecoverTimeElapsed` (`self.staggerRecoverTime`))
        (set `self.damageRecoverTimeElapsed` 0.0)
        ;[1 1 1] Reset damage here
        (if _returnvalue
          (bind _ascharacter (cast `Character` (`self.GetOwner`)))
          (`self.OnStaggerChanged` true)
          (`|PlayMontage` (`Character.Mesh` _ascharacter) _value (/ 1.0 (`self.staggerRecoverTime`))
            (:`OnCompleted`
              (set `self.isStaggered` false)
              (`self.OnStaggerChanged` false))
            (:`OnInterrupted`
              (`KismetSystemLibrary.PrintString` "Anim Interrupted"))))))))

(fn `BPCalculateStaggerChance`
  (returns (StaggerChance :type "Float (double-precision)"))
  (locals (AdditionalPercentToAdd :type "Float (double-precision)"))
  (bind _output_get (set `self.damageDealtForStaggerPurposes` (+ (`self.damageDealtForStaggerPurposes`) (`self.damageDealt`))))
  (bind _output_get_2 (set `local.AdditionalPercentToAdd` (- 1.0 (`KismetMathLibrary.FClamp` (/ (`self.minStaggerChance`) 100.0)))))
  (return (+ (`self.minStaggerChance`) (* (* (`KismetMathLibrary.FClamp` (/ (- _output_get (`self.minDamageToStagger`)) (- (`self.weakSpotDamageGuaranteedStaggerThreshold`) (`self.minDamageToStagger`)))) _output_get_2) 100.0))))