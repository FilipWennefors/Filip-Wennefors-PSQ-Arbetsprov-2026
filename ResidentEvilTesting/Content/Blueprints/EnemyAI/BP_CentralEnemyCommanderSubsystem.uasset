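; BP_CentralEnemyCommanderSubsystem is a central AI subsystem that caps how many enemies engage the player at once.
; TryEngagePlayer grants a BaseEnemy a slot while the engaged count is below the maximum, adding it to EnemiesEngaged and returning whether it succeeded.
; OnEnemyKilled removes the dead enemy from that array and decrements the separately tracked count, freeing the slot.
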(event `self.OnInitializedBP`)

(event `self.OnEnemyKilled`
  (params (EnemyKilled :type "BaseEnemy Object Reference") (bIsReallyDead :type Boolean))
  (for (_array_element _array_index) (`self.EnemiesEngaged`)
    (if (== _array_element EnemyKilled)
      (`KismetArrayLibrary.Array_Remove` (`self.EnemiesEngaged`) _array_index)
      (set `self.EnemiesEngagedCount` (- (`self.EnemiesEngagedCount`) 1.0)))))

(fn `TryEngagePlayer`
  (params (EnemyAskingToEngage :type "Pawn Object Reference"))
  (returns (NewParam :type Boolean))
  (bind _asbase_enemy (cast `BaseEnemy` EnemyAskingToEngage))
  (if (< (`self.EnemiesEngagedCount`) (`self.MaxEnemiesEngagedCount`))
    (`KismetArrayLibrary.Array_AddUnique` (`self.EnemiesEngaged`) _asbase_enemy)
    (set `self.EnemiesEngagedCount` (+ (`self.EnemiesEngagedCount`) 1.0))
    (return true)
    (else
      (return false))))