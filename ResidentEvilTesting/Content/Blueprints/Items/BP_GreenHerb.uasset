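; BP_GreenHerb is a healing item that restores health to the player's third-person character when used from the inventory.
; TryUseItem checks whether the controlled pawn is already at max health and, if not, heals it by HealthAdded.
; It then removes itself through the player inventory subsystem and returns true, while a player at full health keeps the herb and gets false.
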(fn `TryUseItem`
  (params (PlayerController :type "ExtendedPlayerController Object Reference"))
  (returns (ReturnValue :type Boolean))
  (locals (Actor :type "ActorActionUtility Object Reference"))
  (bind _asbp_third_person_character (cast `/Game/Blueprints/Player/BP_ThirdPersonCharacter` (`Controller.K2_GetPawn` PlayerController)))
  (bind _returnvalue (`/Game/Blueprints/Player/BP_ThirdPersonCharacter.IsMaxHealth` _asbp_third_person_character))
  (if (not _returnvalue)
    (`PlayerCharacter.HealPlayer` _asbp_third_person_character (`self.HealthAdded`))
    (bind _returnvalue_2 (`ExtendedPlayerController.GetPlayerInventorySubsystem` PlayerController))
    (bind _asbp_player_inventory_subsystem (cast `/Game/Blueprints/Player/BP_PlayerInventorySubsystem` _returnvalue_2))
    (`PlayerInventorySubsystem.RemoveItemFromInventory` _asbp_player_inventory_subsystem self)
    (return true)
    (else
      (return false))))