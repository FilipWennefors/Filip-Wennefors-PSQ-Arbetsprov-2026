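; BP_TestInteractable is a test interactable object that always allows interaction and destroys itself on any damage.
; StartInteraction casts the player pawn to PlayerCharacter and plays a crate-stomp montage on its mesh through PlayMontageOnPlayerWithCallbacks.
; The damage handler is separate from the interaction, and a few unconnected nodes, including a class-check debug print, never run.
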(event `self.ReceiveBeginPlay`)

(event `self.ReceiveTick`
  (params (DeltaSeconds :type "Float (single-precision)")))

(event `self.StartInteraction`
  (bind _asplayer_character (cast `PlayerCharacter` (`GameplayStatics.GetPlayerPawn` 0)))
  (`PlayMontageOnPlayerWithCallbacks.PlayMontageOnPlayerWithCallbacks` (`Character.Mesh` _asplayer_character) "/Game/Animations/LeonCustomAnimations/Montages/Ue5Rig_Leon_StompCrate_Montage.Ue5Rig_Leon_StompCrate_Montage" 1.0))

(event `self.ReceiveAnyDamage`
  (params (Damage :type "Float (single-precision)") (DamageType :type "DamageType Object Reference") (InstigatedBy :type "Controller Object Reference") (DamageCauser :type "Actor Object Reference"))
  (`self.K2_DestroyActor`))

(fn `CanInteractWithObject`
  (returns (ReturnValue :type Boolean))
  (return true))

(fn `UserConstructionScript`)