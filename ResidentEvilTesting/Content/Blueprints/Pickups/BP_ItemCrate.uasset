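; Breakable item crate that the player can interact with and that drops an item pickup when damaged.
; Starting interaction plays a stomp-crate montage on the player character, and the crate always reports itself as interactable.
; Any damage prints the amount, traces far downward on the Visibility channel to spawn an ItemPickup at the hit point, then destroys the crate, even if the trace misses.
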(event `self.ReceiveAnyDamage`
  (params (Damage :type "Float (single-precision)") (DamageType :type "DamageType Object Reference") (InstigatedBy :type "Controller Object Reference") (DamageCauser :type "Actor Object Reference"))
  (`KismetSystemLibrary.PrintString` (`KismetStringLibrary.BuildString_Double` "Dealt damage: " "" Damage))
  (bind (_outhit _returnvalue) (`KismetSystemLibrary.LineTraceSingle` (`self.K2_GetActorLocation`) (+ (`self.K2_GetActorLocation`) (* (`self.GetActorUpVector`) (1.0 1.0 -100000000.0))) "TraceTypeQuery1"))
  (if _returnvalue
    (`|SpawnActorFromClass` (`self.ItemPickup`) (`KismetMathLibrary.MakeTransform` (`.Location` (`GameplayStatics.BreakHitResult` _outhit))) "Undefined" "OverrideRootScale" null null))
  (`self.K2_DestroyActor`))

(event `self.StartInteraction`
  (bind _asplayer_character (cast `PlayerCharacter` (`GameplayStatics.GetPlayerPawn` 0)))
  (`PlayMontageOnPlayerWithCallbacks.PlayMontageOnPlayerWithCallbacks` (`Character.Mesh` _asplayer_character) "/Game/Animations/LeonCustomAnimations/Montages/Ue5Rig_Leon_StompCrate_Montage.Ue5Rig_Leon_StompCrate_Montage" 1.0))

(event `self.Interact`)

(event `self.OnConfirmedClosestInteractable`)

(fn `CanInteractWithObject`
  (returns (ReturnValue :type Boolean))
  (return true))

(fn `UserConstructionScript`)