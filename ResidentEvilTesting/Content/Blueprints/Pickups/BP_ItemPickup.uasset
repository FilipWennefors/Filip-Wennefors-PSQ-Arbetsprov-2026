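; World item pickup that grants a configured item to the player's inventory when interacted with, then destroys itself.
; It constructs the item on BeginPlay and, on interaction, routes it to the inventory subsystem as a regular or special item.
; An added-item HUD modal shows on first pickup or when no item info exists.
; While confirmed as closest interactable, a camera-facing prompt stays visible via a retriggerable delay.
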(event `self.ReceiveBeginPlay`
  (`SceneComponent.SetVisibility` (`self.Widget`) false false)
  (bind _returnvalue (`|GenericCreateObject` (`self.Item To Grant`)))
  (set `self.ItemToGrantObject` _returnvalue))

(event `self.ReceiveTick`
  (params (DeltaSeconds :type "Float (single-precision)")))

(event `self.OnConfirmedClosestInteractable`
  (`SceneComponent.K2_SetWorldRotation` (`self.Widget`) (`KismetMathLibrary.FindLookAtRotation` (`SceneComponent.K2_GetComponentLocation` (`self.Widget`)) (`PlayerCameraManager.GetCameraLocation` (`GameplayStatics.GetPlayerCameraManager` 0))) false false)
  (`SceneComponent.SetVisibility` (`self.Widget`) true true)
  (`KismetSystemLibrary.RetriggerableDelay` 0.1)
  (`SceneComponent.SetVisibility` (`self.Widget`) false false))

(event `self.Sphere.OnComponentBeginOverlap`
  (params (OverlappedComponent :type "PrimitiveComponent Object Reference") (OtherActor :type "Actor Object Reference") (OtherComp :type "PrimitiveComponent Object Reference") (OtherBodyIndex :type Integer) (bFromSweep :type Boolean) (SweepResult :type "HitResult Structure (by ref)"))
  (`KismetSystemLibrary.PrintString` "Sphere overlap")
  (if (== OtherActor (`GameplayStatics.GetPlayerPawn` 0))
    (set `self.Interactable` true)))

(event `self.Sphere.OnComponentEndOverlap`
  (params (OverlappedComponent :type "PrimitiveComponent Object Reference") (OtherActor :type "Actor Object Reference") (OtherComp :type "PrimitiveComponent Object Reference") (OtherBodyIndex :type Integer))
  (if (== OtherActor (`GameplayStatics.GetPlayerPawn` 0))
    (set `self.Interactable` false)))

(event `self.StartInteraction`
  (bind _returnvalue (subsystem `/Game/Blueprints/Player/BP_PlayerInventorySubsystem`))
  (bind _itemtograntobject (`self.ItemToGrantObject`))
  (if (`KismetSystemLibrary.IsValid` (`self.ItemToGrantObject`))
    (bind _asnew_inventory_item (cast `NewInventoryItem` _itemtograntobject)
      (:`then`
        (bind (_bisitemrotated _outitemposition _returnvalue_2) (`PlayerInventorySubsystem.TryAddItemToInventory` _returnvalue _asnew_inventory_item (`self.Item Quantity`)))
        (if _returnvalue_2
          (`self.Show Item Added Modal` _asnew_inventory_item "/Game/Blueprints/WidgetBlueprints/WBP_ItemAddedModal.WBP_ItemAddedModal_C")
          (`self.K2_DestroyActor` :!label _label)))
      (:`CastFailed`
        (bind _asspecial_item (cast `SpecialItem` _itemtograntobject))
        (bind _returnvalue_3 (`PlayerInventorySubsystem.AddSpecialItemToInventory` _returnvalue _asspecial_item))
        (if _returnvalue_3
          (`self.Show Item Added Modal` _asspecial_item "/Game/Blueprints/WidgetBlueprints/WBP_ItemAddedModal.WBP_ItemAddedModal_C")
          (goto _label))))
    (else
      (`KismetSystemLibrary.PrintString` "ERROR: ITEM TO GRANT IS INVALID"))))

(fn `CanInteractWithObject`
  (returns (ReturnValue :type Boolean))
  (return true))

(fn `Show Item Added Modal`
  (params (ItemAdded :type "Item Object Reference") (ModalClass :type "/Game/Blueprints/WidgetBlueprints/WBP_ItemAddedModal Class Reference"))
  (bind _returnvalue (`KismetSystemLibrary.GetClassDisplayName` (`GameplayStatics.GetObjectClass` ItemAdded)))
  (bind _iteminformation (`PlayerInventorySubsystem.itemInformation` (subsystem `/Game/Blueprints/Player/BP_PlayerInventorySubsystem`)))
  (bind (_value _returnvalue_2) (`BlueprintMapLibrary.Map_Find` _iteminformation _returnvalue))
  (if _returnvalue_2
    (if (`.bFirstTimePickedUp` (break `ItemInfo` _value))
      (bind _structout (setmembers `ItemInfo` :`StructRef` _value :`bFirstTimePickedUp` false))
      (`BlueprintMapLibrary.Map_Add` _iteminformation _returnvalue _structout)
      (bind _asbp_new_player_hud (cast `/Game/Blueprints/Player/BP_NewPlayerHud` (`PlayerController.GetHUD` (`GameplayStatics.GetPlayerController` 0)) :!label _label))
      (`/Game/Blueprints/Player/BP_NewPlayerHud.Show Item Added Modal` _asbp_new_player_hud ModalClass (`Item.itemIconTexture` ItemAdded) (`Item.itemName` ItemAdded) (`Item.itemDescription` ItemAdded)))
    (else
      (goto _label))))

(fn `UserConstructionScript`)