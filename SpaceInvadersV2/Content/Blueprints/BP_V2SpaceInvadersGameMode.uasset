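; Game mode for a Space Invaders game that spawns and drives the invader waves and barracks.
; RestartGame resets state and spawns both grids through SpawnInvaders, placed by camera distance; BeginPlay calls it after a delay, then pauses.
; Tick moves the grid with MoveInvadersV2, storing the returned direction, and respawns a clamped, lower wave once all die.
; Many disconnected chains hold older movement and placement experiments.
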(event `self.ReceiveBeginPlay`
  (`KismetSystemLibrary.Delay` 1.0)
  (`self.RestartGame`)
  (`GameplayStatics.SetGamePaused` true))

(event `self.ReceiveTick`
  (params (DeltaSeconds :type "Float (single-precision)"))
  (set `self.Delta Seconds` DeltaSeconds)
  (if (> (`KismetArrayLibrary.Array_Length` (`self.Spawned Invaders`)) 0)
    (bind _returnvalue (`self.AllInvadersKilled` (`self.InvadersCountHorizontal`) (`self.InvadersCountVertical`)))
    (if _returnvalue
      (set `self.Invaders Vertical Spawn Pos` (`KismetMathLibrary.FClamp` (- (`self.Invaders Vertical Spawn Pos`) 50.0) (`self.MinInvadersVerticalSpawnPos`) (`self.MaxInvadersVerticalSpawnPos`)))
      (bind _asbp_camera_manager (cast `/Game/Blueprints/BP_CameraManager` (`GameplayStatics.GetPlayerCameraManager` 0)))
      (bind _camera_spawn_pos_x (`KismetMathLibrary.BreakVector` (`/Game/Blueprints/BP_CameraManager.Camera Spawn Pos` _asbp_camera_manager)))
      (bind _spawnedinvaders (`self.SpawnInvaders` (`self.Invader Class Reference`) (`self.InvadersCountHorizontal`) (`self.InvadersCountVertical`) (`self.Dist Between Invaders`) (`self.Invaders Vertical Spawn Pos`) (`KismetMathLibrary.Abs` _camera_spawn_pos_x)))
      (set `self.Spawned Invaders` _spawnedinvaders)
      (set `self.Invaders Move Direction` 1.0)
      (else
        (bind _asbp_camera_manager_2 (cast `/Game/Blueprints/BP_CameraManager` (`GameplayStatics.GetPlayerCameraManager` 0)))
        (bind _camera_spawn_pos_x_2 (`KismetMathLibrary.BreakVector` (`/Game/Blueprints/BP_CameraManager.Camera Spawn Pos` _asbp_camera_manager_2)))
        (bind _movedirout (`self.MoveInvadersV2` (`self.Invaders Move Speed`) (`self.Invaders Move Direction`) (`self.InvadersCountHorizontal`) (`self.InvadersCountVertical`) (`KismetMathLibrary.Abs` _camera_spawn_pos_x_2) (`self.Delta Seconds`) (`self.Spawned Invaders`)))
        (set `self.Invaders Move Direction` _movedirout)))))

(fn `RestartGame`
  (set `self.Invaders Vertical Spawn Pos` (`self.MaxInvadersVerticalSpawnPos`))
  (`self.ResetGameState` (`self.Spawned Invaders`) (`self.Spawned Barracks`))
  (bind _asbp_camera_manager (cast `/Game/Blueprints/BP_CameraManager` (`GameplayStatics.GetPlayerCameraManager` 0)))
  (bind _camera_spawn_pos_x (`KismetMathLibrary.BreakVector` (`/Game/Blueprints/BP_CameraManager.Camera Spawn Pos` _asbp_camera_manager)))
  (bind _returnvalue (`KismetMathLibrary.Abs` _camera_spawn_pos_x))
  (bind _spawnedinvaders (`self.SpawnInvaders` (`self.Invader Class Reference`) (`self.InvadersCountHorizontal`) (`self.InvadersCountVertical`) (`self.Dist Between Invaders`) (`self.Invaders Vertical Spawn Pos`) _returnvalue))
  (set `self.Spawned Invaders` _spawnedinvaders)
  (bind _spawnedinvaders_2 (`self.SpawnInvaders` "/Game/Blueprints/Actors/BP_Barracks.BP_Barracks_C" (`self.Barracks Count`) 1 (`self.Dist Between Barracks`) (`self.Barracks Vertical Spawn Pos`) _returnvalue))
  (set `self.Spawned Barracks` _spawnedinvaders_2)
  (set `self.HasSpawnedFirstWave` true)
  (`GameplayStatics.SetGamePaused` false))

(fn `UserConstructionScript`)