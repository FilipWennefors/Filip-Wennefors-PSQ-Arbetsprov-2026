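; BP_PlayerShip is the player's ship in a shooter, with movement, shooting, health and a pause toggle.
; Enhanced Input actions call the move, shoot and pause functions, which are defined outside these graphs.
; A second after BeginPlay, it derives sideways limits from screen corners in world space, using the camera manager's spawn depth.
; Overlapping an enemy bullet deals damage; leftover easing debug code never runs.
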(event `self.ReceiveBeginPlay`
  (`EnhancedInputSubsystemInterface.AddMappingContext` (pcsubsystem `EnhancedInputLocalPlayerSubsystem` (`GameplayStatics.GetPlayerController` 0)) "/Game/Input/IMC_SpaceCraft.IMC_SpaceCraft" 0 (struct))
  (`self.SetPlayerHealth` (`self.BaseHealth`))
  (`KismetSystemLibrary.Delay` 1.0)
  (bind _asbp_v2camera_manager (cast `/Game/Blueprints/BP_CameraManager` (`GameplayStatics.GetPlayerCameraManager` 0)))
  (bind _camera_spawn_pos_x (`KismetMathLibrary.BreakVector` (`/Game/Blueprints/BP_CameraManager.Camera Spawn Pos` _asbp_v2camera_manager)))
  (bind _returnvalue (`KismetMathLibrary.Abs` _camera_spawn_pos_x))
  (bind _returnvalue_2 (`SpaceInvadersCameraManager.GetLeftCornerPosInWorldSpace` _returnvalue))
  (set `self.MinSidewaysPosition` (.y _returnvalue_2))
  (bind _returnvalue_3 (`SpaceInvadersCameraManager.GetRightCornerPosInWorldSpace` _returnvalue))
  (set `self.MaxSidewaysPosition` (.y _returnvalue_3)))

(event `self.ReceiveActorBeginOverlap`
  (params (OtherActor :type "Actor Object Reference"))
  (if (== (`GameplayStatics.GetObjectClass` OtherActor) "/Game/Blueprints/Actors/BP_EnemyBullet.BP_EnemyBullet_C")
    (`self.TakeDamage` 1)))

(event `self.ReceiveTick`
  (params (DeltaSeconds :type "Float (single-precision)"))
  (set `self.Delta Seconds` DeltaSeconds))

(event `EnhancedInput|/Game/Input/MovePlayerShip`
  (params (ActionValue :type "Float (double-precision)") (ElapsedSeconds :type "Float (double-precision)") (TriggeredSeconds :type "Float (double-precision)") (InputAction :type "InputAction Object Reference" :default "/Game/Input/MovePlayerShip.MovePlayerShip"))
  (:`Triggered`
    (`self.MovePlayerShip` (`self.ShipMoveSpeed`) ActionValue)))

(event `EnhancedInput|/Game/Input/Shoot`
  (params (ActionValue :type Boolean) (ElapsedSeconds :type "Float (double-precision)") (TriggeredSeconds :type "Float (double-precision)") (InputAction :type "InputAction Object Reference" :default "/Game/Input/Shoot.Shoot"))
  (:`Triggered`
    (`self.Shoot` (`self.Fire Rate`) (`self.Ship Relative Spawn Pos`))))

(event `EnhancedInput|/Game/Input/TogglePause`
  (params (ActionValue :type Boolean) (ElapsedSeconds :type "Float (double-precision)") (TriggeredSeconds :type "Float (double-precision)") (InputAction :type "InputAction Object Reference" :default "/Game/Input/TogglePause.TogglePause"))
  (:`Started`
    (`self.OnPauseToggled`)))

(fn `UserConstructionScript`)