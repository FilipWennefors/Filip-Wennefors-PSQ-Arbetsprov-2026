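; BP_Invader is an enemy invader that fires at random and dies when hit by a player bullet.
; Tick passes through a half-second Delay, throttling calls to ShootRandomChance with a configurable chance and spawn offset.
; Overlapping BP_PlayerBullet invokes OnInvaderKilled with 100 and destroys the actor.
; Both the overlap and Destroyed events spawn the death effect, so a bullet kill triggers it twice.
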(event `self.ReceiveTick`
  (params (DeltaSeconds :type "Float (single-precision)"))
  (`KismetSystemLibrary.Delay` 0.5)
  (`self.ShootRandomChance` (`self.ShootingPercentageChance`) (`self.Ship Relative Spawn Pos`)))

(event `self.ReceiveActorBeginOverlap`
  (params (OtherActor :type "Actor Object Reference"))
  (if (== (`GameplayStatics.GetObjectClass` OtherActor) "/Game/Blueprints/Actors/BP_PlayerBullet.BP_PlayerBullet_C")
    (`self.InvokeOnInvaderKilled` 100)
    (`self.K2_DestroyActor`)
    (`NiagaraFunctionLibrary.SpawnSystemAtLocation` "/Game/FXE_InvaderDead.FXE_InvaderDead" (`self.K2_GetActorLocation`) (struct :`Yaw` 90.0) (0.1 0.1 0.1))))

(event `self.ReceiveDestroyed`
  (`NiagaraFunctionLibrary.SpawnSystemAtLocation` "/Game/FXE_InvaderDead.FXE_InvaderDead" (`self.K2_GetActorLocation`) (struct :`Yaw` 90.0) (0.1 0.1 0.1)))

(fn `UserConstructionScript`)