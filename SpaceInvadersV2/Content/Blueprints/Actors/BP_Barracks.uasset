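; BP_Barracks is a barracks actor that takes damage from bullets and displays its health on a widget health bar.
; Overlaps with enemy or player bullets, matched by exact class, call TakeDamage with a fixed amount, higher for player bullets.
; The UpdateHealthBar event casts the widget component's widget to WBP_BarrackHealthBar and sets its progress bar to new health over MaxHealth.
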(event `self.ReceiveActorBeginOverlap`
  (params (OtherActor :type "Actor Object Reference"))
  (if (== (`GameplayStatics.GetObjectClass` OtherActor) "/Game/Blueprints/Actors/BP_EnemyBullet.BP_EnemyBullet_C")
    (`self.TakeDamage` 1)
    (elif (== (`GameplayStatics.GetObjectClass` OtherActor) "/Game/Blueprints/Actors/BP_PlayerBullet.BP_PlayerBullet_C")
      (`self.TakeDamage` 3))))

(event `self.UpdateHealthBar`
  (params (newHealth :type Integer))
  (bind _aswbp_barrack_health_bar (cast `/Game/Blueprints/WidgetBlueprints/WBP_BarrackHealthBar` (`WidgetComponent.GetWidget` (`self.Widget`))))
  (`ProgressBar.SetPercent` (`/Game/Blueprints/WidgetBlueprints/WBP_BarrackHealthBar.ProgressBar_48` _aswbp_barrack_health_bar) (/ newHealth (`self.MaxHealth`))))

(fn `UserConstructionScript`)