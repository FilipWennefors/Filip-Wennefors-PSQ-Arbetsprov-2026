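; BP_EnemyBullet is an enemy projectile actor that destroys itself when it hits the player ship or a barracks.
; ActorBeginOverlap compares the other actor's exact class to BP_PlayerShip and BP_Barracks, ignoring anything else.
; The graph applies no damage and has no movement logic; BeginPlay only assigns MoveSpeed to itself, and Tick is disabled.
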(event `self.ReceiveBeginPlay`
  (set `self.moveSpeed` (`self.Move Speed`)))

(event `self.ReceiveActorBeginOverlap`
  (params (OtherActor :type "Actor Object Reference"))
  (if (== (`GameplayStatics.GetObjectClass` OtherActor) "/Game/Blueprints/Actors/BP_PlayerShip.BP_PlayerShip_C")
    (`self.K2_DestroyActor`)
    (elif (== (`GameplayStatics.GetObjectClass` OtherActor) "/Game/Blueprints/Actors/BP_Barracks.BP_Barracks_C")
      (`self.K2_DestroyActor`))))

(fn `UserConstructionScript`)